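; Actor component that runs dialogue and timed decisions for its player character, driving the WB_MainDialogue widget and reporting results back to the NPC.
; Dialogue lines play sound and text, then continue automatically or on input, with optional skipping.
; Decisions enable mouse and number-key selection, submitting the current selection when any time limit expires.
; Server, owning-client and multicast events handle widgets, choices, teleporting and the NPC busy state.
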(event Custom|AddSimpleDialogue%20-ALL
  (params (Dialogue :type S%20Dialogue%20Info%20Structure) (Index :type Integer))
  (bind _dialoguewidget (Variables|Widget|GetDialogueWidget))
  ;[1 1 1] Add Simple Dialogue
  (Variables|Default|SetCurrentDialogue Dialogue)
  (if (not (Variables|Default|GetDialogue))
    (Variables|Default|SetDialogue true)
    (Variables|Default|SetIndex Index)
    (Utilities|IsValid (.Sound (Utilities|Struct|BreakS_DialogueInfo (Variables|Default|GetCurrentDialogue)))
      (:Is%20Valid
        (bind _returnvalue (Audio|SpawnSoundatLocation (.Sound (Utilities|Struct|BreakS_DialogueInfo (Variables|Default|GetCurrentDialogue))) (Transformation|GetActorLocation (Components|GetOwner)) "0, 0, 0" 1.0 1.0 0.0 0 0))
        (Variables|Default|SetCurrentSound _returnvalue))
      (:Is%20Not%20Valid
        _))
    (Utilities|IsValid (Variables|Widget|GetDialogueWidget)
      (:Is%20Valid
        (Default|ShowNewMessage (Variables|Widget|GetDialogueWidget) (.Speaker (Utilities|Struct|BreakS_DialogueInfo (Variables|Default|GetCurrentDialogue))) (.Dialogue (Utilities|Struct|BreakS_DialogueInfo (Variables|Default|GetCurrentDialogue)))))
      (:Is%20Not%20Valid
        _))
    (Utilities|FlowControl|Sequence
      (:then_0
        (if (.Skippable (Utilities|Struct|BreakS_DialogueInfo (Variables|Default|GetCurrentDialogue)))
          (Utilities|FlowControl|Delay (.SkipTime (Utilities|Struct|BreakS_DialogueInfo (Variables|Default|GetCurrentDialogue))))
          (Variables|Default|SetWInput true)
          (Utilities|IsValid _dialoguewidget
            (:Is%20Valid
              (Default|SetSkipVisiable _dialoguewidget "SelfHitTestInvisible")))))
      (:then_1
        (bind _returnvalue_2 (Utilities|Time|SetTimerbyEvent (delegate Custom|OnDialogueSpoken) (select (Utilities|IsValid (.Sound (Utilities|Struct|BreakS_DialogueInfo (Variables|Default|GetCurrentDialogue)))) (Variables|/Script/Engine.SoundBase|GetDuration (.Sound (Utilities|Struct|BreakS_DialogueInfo (Variables|Default|GetCurrentDialogue)))) 1.0)))
        (Variables|Default|SetOptionsTimer _returnvalue_2)))))

(event Custom|RemoveWidget%20-ALL
  (bind _mainwidget (Variables|Widget|GetMainWidget))
  (bind _playercontroller (Variables|References|GetPlayerController))
  ;[1 1 1] Replicate Busy State
  (Utilities|IsValid _mainwidget
    (:Is%20Valid
      (Widget|RemovefromParent _mainwidget))
    (:Is%20Not%20Valid
      _))
  (Utilities|IsValid _playercontroller
    (:Is%20Valid
      ;[1 1 1] Create Dialogue Widget
      (Input|SetInputModeGameOnly _playercontroller false))))

(event Custom|CreateWidget%20-OC
  ;[1 1 1] Create Dialogue Widget
  (bind _returnvalue (UserInterface|CreateWidget "/Game/ModernRPG/General/GUI/Widgets/DialoguesQuests/Dialogue/WB_MainDialogue.WB_MainDialogue_C"))
  (bind _output_get (Variables|Widget|SetMainWidget _returnvalue))
  (Variables|Widget|SetDialogueWidget (Variables|/Game/ModernRPG/General/GUI/Widgets/DialoguesQuests/Dialogue/WB_MainDialogue.WB_MainDialogue_C|GetDialogueWidget _output_get))
  (Variables|Widget|SetDecisionWidget (Variables|/Game/ModernRPG/General/GUI/Widgets/DialoguesQuests/Dialogue/WB_MainDialogue.WB_MainDialogue_C|GetDecisionWidget (Variables|Widget|GetMainWidget)))
  (Variables|/Game/ModernRPG/General/GUI/Widgets/DialoguesQuests/Dialogue/WB_TimerDialogue.WB_TimerDialogue_C|SetDialogueManager (Variables|/Game/ModernRPG/General/GUI/Widgets/DialoguesQuests/Dialogue/WB_MainDialogue.WB_MainDialogue_C|GetDecisionWidget (Variables|Widget|GetMainWidget)) self))

(event Custom|TeleportPlayer%20-Server
  (params (NewLocation :type Vector) (NewRotation :type Rotator))
  ;[1 1 1] Teleport Player to the Location Replicated
  (CallFunction|TeleportPlayer-ALL NewLocation NewRotation))

(event Custom|RemoveWidget
  ;[1 1 1] Replicate Busy State
  (if (Ability|HasAuthority (Components|GetOwner))
    (CallFunction|RemoveWidget-ALL)
    (else
      (CallFunction|RemoveWidget-Server))))

(event Custom|TeleportPlayer%20-ALL
  (params (NewLocation :type Vector) (NewRotation :type Rotator))
  (bind _returnvalue (Components|GetOwner))
  ;[1 1 1] Teleport Player to the Location Replicated
  (Transformation|SetActorLocation _returnvalue NewLocation false true)
  (Transformation|SetActorRotation _returnvalue NewRotation))

(event Custom|AddSimpleDialogue%20-Server
  (params (Dialogue :type S%20Dialogue%20Info%20Structure) (Index :type Integer))
  ;[1 1 1] Add Simple Dialogue
  (CallFunction|AddSimpleDialogue-ALL Dialogue Index))

(event Custom|ShowWidget
  ;[1 1 1] Create Dialogue Widget
  (if (Ability|HasAuthority (Components|GetOwner))
    (CallFunction|ShowWidget-OC)
    (else
      (CallFunction|ShowWidget-Server))))

(event Custom|ShowWidget%20-Server
  ;[1 1 1] Create Dialogue Widget
  (CallFunction|ShowWidget-OC))

(event Custom|ToggleBusy%20-Server
  (params (Busy :type Boolean) (Character :type BP%20Dialogue%20Character%20Object%20Reference))
  ;[1 1 1] Toggle Player's State
  (CallFunction|ToggleBusy-ALL Busy Character)
  (if Busy
    (Actor|SetOwner Character (Components|GetOwner))
    (else
      (Actor|SetOwner Character 0)
      (CallFunction|ShowCharacterInfo-ALL Character))))

(event Custom|CreateWidget
  ;[1 1 1] Create Dialogue Widget
  (if (Ability|HasAuthority (Components|GetOwner))
    (CallFunction|CreateWidget-OC)
    (else
      (CallFunction|CreateWidget-Server))))

(event Custom|ToggleBusy%20-ALL
  (params (Busy :type Boolean) (Character :type BP%20Dialogue%20Character%20Object%20Reference))
  ;[1 1 1] Toggle Player's State
  (Variables|/Game/ModernRPG/General/Blueprints/DialoguesQuests/Dialogue/BP_DialogueCharacter.BP_DialogueCharacter_C|SetBusy Character Busy))

(event Custom|ToggleBusy
  (params (Busy :type Boolean) (Character :type BP%20Dialogue%20Character%20Object%20Reference))
  ;[1 1 1] Toggle Busy in Dialogue Charcter
  (if (Ability|HasAuthority (Components|GetOwner))
    (CallFunction|ToggleBusy-ALL Busy Character)
    (else
      (CallFunction|ToggleBusy-Server Busy Character))))

(event Custom|CreateWidget%20-Server
  ;[1 1 1] Create Dialogue Widget
  (CallFunction|CreateWidget-OC))

(event Custom|RemoveWidget%20-Server
  ;[1 1 1] Replicate Busy State
  (CallFunction|RemoveWidget-ALL))

(event Custom|ShowWidget%20-OC
  (bind _mainwidget (Variables|Widget|GetMainWidget))
  ;[1 1 1] Create Dialogue Widget
  (Utilities|IsValid (Variables|Widget|GetMainWidget)
    (:Is%20Valid
      (if (not (UserInterface|Viewport|IsinViewport _mainwidget))
        (UserInterface|Viewport|AddtoViewport _mainwidget 0)
        (Class|Widget|SetUserFocus _mainwidget (Variables|References|GetPlayerController))
        (Input|SetInputModeUIOnly (Variables|References|GetPlayerController) _mainwidget "DoNotLock" false)))))

(event Custom|OnDialogueSpoken
  (bind _dialoguewidget (Variables|Widget|GetDialogueWidget))
  (bind _currentsound (Variables|Default|GetCurrentSound))
  ;[1 1 1] On Dialogue Spoken
  (if (and (not (Variables|Default|GetDone)) (Variables|Default|GetDialogue))
    (Variables|Default|SetDone true)
    (Variables|Default|SetWInput true)
    (Utilities|IsValid _dialoguewidget
      (:Is%20Valid
        (Default|SetSkipVisiable _dialoguewidget "Hidden"))
      (:Is%20Not%20Valid
        _))
    (Utilities|IsValid _currentsound
      (:Is%20Valid
        (Audio|Components|Audio|Stop _currentsound)
        (Components|DestroyComponent _currentsound))
      (:Is%20Not%20Valid
        _))
    (if (.PressToContinue? (Utilities|Struct|BreakS_DialogueInfo (Variables|Default|GetCurrentDialogue)))
      (Default|SetContinueVisiable (Variables|Widget|GetDialogueWidget) "Visible")
      (else
        (CallFunction|HandleContinueCommand)
        (Utilities|Time|PauseTimerbyHandle (Variables|Default|GetOptionsTimer))))))

(event Custom|ShowCharacterInfo%20-ALL
  (params (Target :type BP%20Dialogue%20Character%20Object%20Reference))
  ;[1 1 1] Show Information
  (Development|SetHiddeninGame (Variables|/Game/ModernRPG/General/Blueprints/DialoguesQuests/Dialogue/BP_DialogueCharacter.BP_DialogueCharacter_C|GetCharacterInfo Target) false false))

(event EventBeginPlay
  ;[1 1 1] Event Begin Play
  (bind _ascharacter (Utilities|Casting|CastToCharacter (Components|GetOwner)))
  (bind _output_get (Variables|References|SetCharacter _ascharacter))
  (bind _asplayer_controller (Utilities|Casting|CastToPlayerController (Pawn|GetController _output_get)))
  (Variables|References|SetPlayerController _asplayer_controller)
  (CallFunction|CreateWidget))

(event Custom|ChooseNumber
  (params (PressedNumber :type Integer))
  ;[1 1 1] Number Keys
  (bind _output_get (Variables|Default|SetCurOption PressedNumber))
  (CallFunction|HandleNumberKey _output_get))

(fn FadeDialogue
  (params (Index :type Boolean))
  (Utilities|IsValid (Variables|References|GetPlayerController)
    (:Is%20Valid
      (if Index
        (CameraFades|StartCameraFade :self (Variables|/Script/Engine.PlayerController|GetPlayerCameraManager (Variables|References|GetPlayerController)) :FromAlpha 1.0 :Duration 2.0)
        (else
          (CameraFades|StartCameraFade :self (Variables|/Script/Engine.PlayerController|GetPlayerCameraManager (Variables|References|GetPlayerController)) :ToAlpha 1.0 :Duration 2.0))))))

(fn IsOptionBlocked
  (params (Index :type Integer))
  (return (Utilities|Enum|NotEqual(Enum) (Variables|/Game/ModernRPG/General/GUI/Widgets/DialoguesQuests/Dialogue/WB_DialogueOptionSLot.WB_DialogueOptionSLot_C|GetCategory (Utilities|Array|Get(acopy) (Variables|/Game/ModernRPG/General/GUI/Widgets/DialoguesQuests/Dialogue/WB_TimerDialogue.WB_TimerDialogue_C|GetOptionWidgets (Variables|Widget|GetDecisionWidget)) (- Index 1))) "NewEnumerator3")))

(event Custom|MulticastSetFinished
  (params (Finished :type Boolean))
  (Variables|Default|SetFinished Finished)
  (Variables|Default|SetDecision Finished))

(event Custom|ServerSetFinished
  (params (Finished :type Boolean))
  (CallFunction|MulticastSetFinished Finished))

(event Custom|OnDecisionMade%20-Server
  (params (OptionIndex :type Integer))
  ;[1 1 1] End Of the Dialogue
  ;;[1 1 1] On Decision Made
  (CallFunction|OnDecisionMade-ALL OptionIndex))

(event Custom|IncreaseFloat
  ;[1 1 1] End Of the Dialogue
  ;;[1 1 1] On Decison Spoken
  ;;;[1 1 1] Increase Float
  (Variables|Time|SetCurTime (+ (Variables|Time|GetCurTime) (Variables|Time|GetMaxTime)))
  (Progress|SetPercent (Variables|/Game/ModernRPG/General/GUI/Widgets/DialoguesQuests/Dialogue/WB_TimerDialogue.WB_TimerDialogue_C|GetTimerBar (Variables|Widget|GetDecisionWidget)) (- 1.0 (/ (Variables|Time|GetCurTime) (Math|Conversions|ToFloat(Integer) (Variables|Time|GetTimer))))))

(event Custom|IncreaseInt
  ;[1 1 1] End Of the Dialogue
  ;;[1 1 1] On Decison Spoken
  ;;;[1 1 1] Increase Int
  (Variables|Time|SetCurTimerSec (+ (Variables|Time|GetCurTimerSec) 1))
  (Rendering|Components|TextRender|SetText (Variables|/Game/ModernRPG/General/GUI/Widgets/DialoguesQuests/Dialogue/WB_TimerDialogue.WB_TimerDialogue_C|GetCounter (Variables|Widget|GetDecisionWidget)) (Utilities|Text|ToText(Integer) (- (Variables|Time|GetTimer) (Variables|Time|GetCurTimerSec))))
  (if (>= (Variables|Time|GetCurTimerSec) (Variables|Time|GetTimer))
    (CallFunction|OnDecisionMade-Server (Variables|/Game/ModernRPG/General/GUI/Widgets/DialoguesQuests/Dialogue/WB_TimerDialogue.WB_TimerDialogue_C|GetCurrentSelectedIndex (Variables|Widget|GetDecisionWidget)))))

(event Custom|OnDecisionSpoken
  (bind _decisionwidget (Variables|Widget|GetDecisionWidget))
  (bind _currentsound (Variables|Default|GetCurrentSound))
  (bind _decisionwidget_2 (Variables|Widget|GetDecisionWidget))
  (bind _decisionwidget_3 (Variables|Widget|GetDecisionWidget))
  (bind _decisionwidget_4 (Variables|Widget|GetDecisionWidget))
  (bind _playercontroller (Variables|References|GetPlayerController))
  (bind _decisioninfo (Variables|/Game/ModernRPG/General/GUI/Widgets/DialoguesQuests/Dialogue/WB_TimerDialogue.WB_TimerDialogue_C|GetDecisionInfo _decisionwidget_3))
  (bind (_dialogue _options _hastimelimit_ _timelimit) (Utilities|Struct|BreakS_Option _decisioninfo))
  ;[1 1 1] End Of the Dialogue
  ;;[1 1 1] On Decison Spoken
  (if (and (not (Variables|Default|GetFinished)) (Variables|Default|GetDecision))
    (Utilities|IsValid (Variables|Widget|GetDecisionWidget)
      (:Is%20Valid
        (Variables|Default|SetFinished true)
        (Variables|Default|SetWInput true)
        (Utilities|IsValid _decisionwidget_4
          (:Is%20Valid
            (Widget|SetVisibility (Variables|/Game/ModernRPG/General/GUI/Widgets/DialoguesQuests/Dialogue/WB_TimerDialogue.WB_TimerDialogue_C|GetOptionsBox _decisionwidget_4) "Visible"))
          (:Is%20Not%20Valid
            _))
        (Utilities|IsValid (Variables|References|GetPlayerController)
          (:Is%20Valid
            (Variables|/Script/Engine.PlayerController|SetbEnableClickEvents (Variables|References|GetPlayerController) true)
            (Variables|/Script/Engine.PlayerController|SetbShowMouseCursor (Variables|References|GetPlayerController) true)
            (Variables|/Script/Engine.PlayerController|SetbEnableMouseOverEvents (Variables|References|GetPlayerController) true))
          (:Is%20Not%20Valid
            _))
        (if _hastimelimit_
          (Widget|SetVisibility (Variables|/Game/ModernRPG/General/GUI/Widgets/DialoguesQuests/Dialogue/WB_TimerDialogue.WB_TimerDialogue_C|GetTimerVB _decisionwidget) "Visible")
          (Rendering|Components|TextRender|SetText (Variables|/Game/ModernRPG/General/GUI/Widgets/DialoguesQuests/Dialogue/WB_TimerDialogue.WB_TimerDialogue_C|GetCounter _decisionwidget) (Utilities|Text|ToText(Integer) _timelimit))
          (Progress|SetPercent (Variables|/Game/ModernRPG/General/GUI/Widgets/DialoguesQuests/Dialogue/WB_TimerDialogue.WB_TimerDialogue_C|GetTimerBar _decisionwidget) 1.0)
          (Variables|Time|SetCurTime 0.0)
          (Variables|Time|SetTimer _timelimit)
          (Variables|Time|SetCurTimerSec 0)
          (bind _returnvalue (Utilities|Time|SetTimerbyEvent (delegate Custom|IncreaseFloat) (Variables|Time|GetMaxTime) true))
          (Variables|Default|SetMainTimer _returnvalue)
          (bind _returnvalue_2 (Utilities|Time|SetTimerbyEvent (delegate Custom|IncreaseInt) 1.0 true))
          (Variables|Default|SetSecondTimer _returnvalue_2))
        (Utilities|IsValid (Variables|Widget|GetDecisionWidget)
          (:Is%20Valid
            (Input|SetInputModeUIOnly _playercontroller _decisionwidget_2 "DoNotLock" false)
            (Class|Widget|SetUserFocus _decisionwidget_2 _playercontroller))
          (:Is%20Not%20Valid
            _))
        (Utilities|IsValid _currentsound
          (:Is%20Valid
            (Audio|Components|Audio|Stop _currentsound)
            (Components|DestroyComponent _currentsound)))))))

(event Custom|OnDecisionMade%20-ALL
  (params (OptionIndex :type Integer))
  (bind _npc (Variables|References|GetNPC))
  ;[1 1 1] End Of the Dialogue
  ;;[1 1 1] On Decision Made
  (Utilities|FlowControl|DoOnce false
    (:Completed
      (Variables|Default|SetChosenOption OptionIndex)
      (Utilities|Time|ClearandInvalidateTimerbyHandle (Variables|Default|GetSecondTimer))
      (Variables|Default|SetWInput false)
      (Utilities|Time|ClearandInvalidateTimerbyHandle (Variables|Default|GetMainTimer))
      (Widget|SetVisibility (Variables|/Game/ModernRPG/General/GUI/Widgets/DialoguesQuests/Dialogue/WB_TimerDialogue.WB_TimerDialogue_C|GetOptionsBox (Variables|Widget|GetDecisionWidget)) "Hidden")
      (Variables|/Script/Engine.PlayerController|SetbEnableClickEvents (Variables|References|GetPlayerController) false)
      (Variables|/Script/Engine.PlayerController|SetbShowMouseCursor (Variables|References|GetPlayerController) false)
      (Variables|/Script/Engine.PlayerController|SetbEnableMouseOverEvents (Variables|References|GetPlayerController) false)
      (Utilities|FlowControl|Delay (Class|WidgetAnimation|GetEndTime (Variables|/Game/ModernRPG/General/GUI/Widgets/DialoguesQuests/Dialogue/WB_TimerDialogue.WB_TimerDialogue_C|GetBlendIn (Variables|Widget|GetDecisionWidget))))
      (Widget|SetVisibility (Variables|Widget|GetDecisionWidget) "Hidden")
      (CallFunction|ServerSetFinished false)
      (Utilities|IsValid _npc
        (:Is%20Valid
          (Default|MadeDecision-Server _npc (Variables|Default|GetCurrentDecisionIndex) (+ (Variables|Default|GetChosenOption) 1)))
        (:Is%20Not%20Valid
          _))
      (CallFunction|ResetDecisionDoOnce))))

(event Custom|ResetDecisionDoOnce
  (bind _npc (Variables|References|GetNPC))
  ;[1 1 1] End Of the Dialogue
  ;;[1 1 1] On Decision Made
  (Utilities|FlowControl|DoOnce false) ; enters at Reset
)

(event Custom|AddDecision
  (params (Decision :type S%20Option%20Structure) (Index :type Integer))
  (bind _dialogue (Utilities|Struct|BreakS_Option Decision))
  (bind _decisionwidget (Variables|Widget|GetDecisionWidget))
  (bind (_sound _dialogue_2 _speaker _skippable _presstocontinue_ _skiptime) (Utilities|Struct|BreakS_DialogueInfo _dialogue))
  ;[1 1 1] Add Decison Dialogue
  (if (not (Variables|Default|GetDecision))
    (Variables|Default|SetDecision true)
    (Variables|Default|SetCurrentDecisionIndex Index)
    (Utilities|IsValid _sound
      (:Is%20Valid
        (bind _returnvalue (Audio|SpawnSoundatLocation _sound (Transformation|GetActorLocation (Components|GetOwner)) "0, 0, 0" 1.0 1.0 0.0 0 0))
        (Variables|Default|SetCurrentSound _returnvalue))
      (:Is%20Not%20Valid
        _))
    (Utilities|IsValid _decisionwidget
      (:Is%20Valid
        (Default|UpdateDialogue _decisionwidget Decision))
      (:Is%20Not%20Valid
        _))
    (Utilities|FlowControl|Sequence
      (:then_0
        (if _skippable
          (Utilities|FlowControl|Delay _skiptime)
          (Variables|Default|SetWInput true)))
      (:then_1
        (Utilities|IsValid _sound
          (:Is%20Valid
            (Utilities|FlowControl|Delay (Variables|/Script/Engine.SoundBase|GetDuration _sound))
            (CallFunction|OnDecisionSpoken))
          (:Is%20Not%20Valid
            (Utilities|FlowControl|Delay 0.5)
            (CallFunction|OnDecisionSpoken)))))))

(event Custom|HandleContinueCommand
  (bind _dialoguewidget (Variables|Widget|GetDialogueWidget))
  (bind _decisionwidget (Variables|Widget|GetDecisionWidget))
  ;[1 1 1] Handle Input Commands
  ;;[1 1 1] Handle Continue Command
  (if (Variables|Default|GetWInput)
    (Utilities|IsValid _dialoguewidget
      (:Is%20Valid
        (Default|SetContinueVisiable _dialoguewidget "Hidden"))
      (:Is%20Not%20Valid
        _))
    (if (Variables|Default|GetDialogue)
      (if (Variables|Default|GetDone)
        (CallFunction|OnContinueDialogue)
        (else
          (CallFunction|OnDialogueSpoken)))
      (elif (Variables|Default|GetFinished)
        (Utilities|IsValid _decisionwidget
          (:Is%20Valid
            (CallFunction|OnDecisionMade-Server (Variables|/Game/ModernRPG/General/GUI/Widgets/DialoguesQuests/Dialogue/WB_TimerDialogue.WB_TimerDialogue_C|GetCurrentSelectedIndex _decisionwidget))))
        (else
          (CallFunction|OnDecisionSpoken))))))

(event Custom|HandleNumberKey
  (params (Number :type Integer))
  (bind _returnvalue (- Number 1))
  (bind _decisionwidget (Variables|Widget|GetDecisionWidget))
  ;[1 1 1] Handle Input Commands
  ;;[1 1 1] Handle Number Keys (0-9)
  (if (Math|Boolean|ANDBoolean (Variables|Default|GetWInput) (Variables|Default|GetFinished) (Variables|Default|GetDecision) (CallFunction|IsOptionBlocked Number))
    (if (and (> Number 0) (<= Number (Utilities|Array|Length (Variables|/Game/ModernRPG/General/GUI/Widgets/DialoguesQuests/Dialogue/WB_TimerDialogue.WB_TimerDialogue_C|GetOptionWidgets _decisionwidget))))
      (Variables|Default|SetWInput false)
      (Default|SelectOption _decisionwidget _returnvalue)
      (CallFunction|OnDecisionMade-Server _returnvalue))))

(event Custom|OnContinueDialogue
  (bind _dialoguewidget (Variables|Widget|GetDialogueWidget))
  (bind _npc (Variables|References|GetNPC))
  (bind _blendin (Variables|/Game/ModernRPG/General/GUI/Widgets/DialoguesQuests/Dialogue/WB_DialogueSlot.WB_DialogueSlot_C|GetBlendIn _dialoguewidget))
  ;[1 1 1] Handle Input Commands
  ;;[1 1 1] On Continue Dialogue
  (Variables|Default|SetWInput false)
  (Utilities|IsValid _dialoguewidget
    (:Is%20Valid
      (UserInterface|Animation|PlayAnimation _dialoguewidget _blendin 0.0 1 "Reverse" 1.0 false)
      (Utilities|FlowControl|Delay (Class|WidgetAnimation|GetEndTime _blendin))
      (Widget|SetVisibility (Variables|Widget|GetDialogueWidget) "Hidden"))
    (:Is%20Not%20Valid
      _))
  (Variables|Default|SetDone false)
  (Variables|Default|SetDialogue false)
  (Utilities|IsValid _npc
    (:Is%20Valid
      (Default|CurrentDialogueFinished _npc (Variables|Default|GetIndex)))))