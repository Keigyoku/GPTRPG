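; Character component that lets its owner climb up or vault over ledges.
; While activated, Tick sphere-traces forward and downward for a ledge, then checks pelvis height and clearance before choosing a climb-up or jump-over montage by height.
; The capsule moves to the computed spot in Flying mode with collision and input off until a montage notify restores walking.
; Server-to-all events replicate movement mode, parkour state and montage; higher climbs temporarily holster weapons.
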(event Custom|StartClimbing
  (params (Value :type Float%20%28double-precision%29) (Location :type Vector) (Height :type Float%20%28double-precision%29))
  (bind _animinstance (GetComponents|GetAnimInstance))
  (bind _climbupedge (Variables|Settings|GetClimbUpEdge))
  (bind _returnvalue (> Height _climbupedge))
  ;[1 1 1] Stick To The Collision
  (if (not (Variables|State|GetParkour))
    (bind _output_get (Variables|State|SetParkour true))
    (CallFunction|ReplicateJumping _output_get)
    (Variables|Engine|SetBlockMovement true)
    (Utilities|IsValid (.Mesh (GetComponents|GetOwnerMesh))
      (:Is%20Valid
        (Utilities|IsValid _animinstance
          (:Is%20Valid
            (Class|BPIClimbInterface|CanClimb(Message) _animinstance true)
            (Default|CallOnClimbingStarted)
            (CallFunction|ReplicateMovement (GetComponents|GetOwnerCharacterMovement) "MOVE_Flying")
            (bind _output_get_2 (Variables|State|SetHanging true))
            (Class|BPIClimbInterface|SetClimbState(Message) (GetComponents|GetAnimInstance) _output_get_2)
            (if _returnvalue
              (bind _output_get_3 (Variables|Engine|SetWasHolstered (CallFunction|IsHolstered? (Components|GetOwner))))
              (if _output_get_3
                _
                (else
                  (CallFunction|ForceToggleWeapon (Components|GetOwner) true)))
              (else
                (Variables|Engine|SetWasHolstered true)))
            (CallFunction|PlayMontageReplicated (select _returnvalue (Variables|Animations|GetAM_ClimbUp) (Variables|Animations|GetAM_JumpOver)) 1.0 Location (Math|Rotator|MakeRotator 0.0 0.0 (- (.Yaw (Math|Rotator|BreakRotator (Math|Conversions|RotationFromXVector (Variables|Engine|GetCollisionNormal)))) Value)))))))))

(event Custom|ClimbJumpEvent
  ;[1 1 1] Trace to Find Grab Object
  (CallFunction|CeClimbOverObject))

(event Custom|ReplicateJumping%20-Server
  (params (Jumping :type Boolean))
  (CallFunction|ReplicateJumping-ALL Jumping))

(event Custom|ReplicateJumping%20-ALL
  (params (Jumping :type Boolean))
  (Variables|State|SetParkour Jumping))

(event Custom|ActivateComponent
  ;[1 1 1] Trace to Find Grab Object
  (if (CallFunction|CanbeClimbing)
    (Components|Tick|SetComponentTickEnabled true)
    (Utilities|FlowControl|Gate true) ; enters at Open
  ))

(event Custom|DeactivateComponent
  ;[1 1 1] Trace to Find Grab Object
  (Components|Tick|SetComponentTickEnabled false)
  (Utilities|FlowControl|Gate true) ; enters at Close
)

(event Custom|StopClimbing
  ;[1 1 1] Stop Climbing
  (if (Variables|State|GetHanging)
    (CallFunction|ReplicateMovement (GetComponents|GetOwnerCharacterMovement) "MOVE_Walking")
    (Variables|State|SetHanging false)
    (Variables|State|SetClimbing false)
    (Utilities|FlowControl|Delay 0.0)
    (Default|ChangeWalkSpeed (Actor|GetComponentbyClass (Components|GetOwner) "/Game/ModernRPG/General/Blueprints/ActorComponents/SpeedChange/AC_SpeedChange.AC_SpeedChange_C") "NewEnumerator0")
    (CallFunction|DeactivateComponent)))

(event Custom|ReplicateMovement
  (params (Target :type Character%20Movement%20Component%20Object%20Reference) (NewMovementMode :type EMovementMode%20Enum :default "MOVE_None"))
  ;[1 1 1] Replicate Movement Mode
  (Networking|SwitchHasAuthority
    (:Authority
      (CallFunction|ReplicateMovement-ALL Target NewMovementMode))
    (:Remote
      (CallFunction|ReplicateMovement-Server Target NewMovementMode))))

(event Custom|ReplicateMovement%20-Server
  (params (Target :type Character%20Movement%20Component%20Object%20Reference) (NewMovementMode :type EMovementMode%20Enum :default "MOVE_None"))
  ;[1 1 1] Replicate Movement Mode
  (CallFunction|ReplicateMovement-ALL Target NewMovementMode))

(event Custom|ClimbBack
  ;[1 1 1] Climb Back
  (if (not (Variables|State|GetClimbing))
    (Utilities|FlowControl|Delay 0.2)
    (Class|BPIClimbInterface|ClimbBackObject(Message) (GetComponents|GetAnimInstance) true)
    (Pawn|Components|CharacterMovement|SetMovementMode (GetComponents|GetOwnerCharacterMovement) "MOVE_Flying" 0)
    (Variables|State|SetClimbing true)
    (Variables|State|SetHanging false)
    (Class|BPIClimbInterface|SetClimbState(Message) (GetComponents|GetAnimInstance) false)))

(event Custom|ceClimbOverObject
  ;[1 1 1] Start Climbing Over The Obgect You Hanging At
  (if (and (not (Variables|State|GetClimbing)) (Variables|Engine|GetCanClimbOver))
    (Class|BPIClimbInterface|ClimbOverObject(Message) (GetComponents|GetAnimInstance) true)
    (Pawn|Components|CharacterMovement|SetMovementMode (GetComponents|GetOwnerCharacterMovement) "MOVE_Flying" 0)
    (Variables|State|SetClimbing true)
    (Variables|State|SetHanging false)
    (Class|BPIClimbInterface|SetClimbState(Message) (GetComponents|GetAnimInstance) false)))

(event Custom|ReplicateMovement%20-ALL
  (params (Target :type Character%20Movement%20Component%20Object%20Reference) (NewMovementMode :type EMovementMode%20Enum :default "MOVE_None"))
  ;[1 1 1] Replicate Movement Mode
  (Pawn|Components|CharacterMovement|SetMovementMode Target NewMovementMode 0))

(event Custom|ReplicateJumping
  (params (State :type Boolean))
  (if (Ability|HasAuthority (Components|GetOwner))
    (CallFunction|ReplicateJumping-ALL State)
    (else
      (CallFunction|ReplicateJumping-Server State))))

(event EventBeginPlay
  ;[1 1 1] Initialize
  (CallFunction|Initialize))

(event EventTick
  (params (DeltaSeconds :type Float%20%28single-precision%29))
  ;[1 1 1] Trace to Find Grab Object
  (Utilities|FlowControl|Gate true
    (:Exit
      (Utilities|MTraceForward
        (:Hit
          (Trace|TraceHeight))))))

(event EventClimbOverObject
  (params (Climbing :type Boolean))
  ;[1 1 1] Finish Climbing over Object
  (Variables|State|SetClimbing Climbing)
  (Pawn|Components|CharacterMovement|SetMovementMode (GetComponents|GetOwnerCharacterMovement) "MOVE_Walking" 0)
  (Utilities|FlowControl|Delay 0.2)
  (Pawn|Components|CharacterMovement|SetMovementMode (GetComponents|GetOwnerCharacterMovement) "MOVE_Walking" 0))

(fn TraceHeight
  (bind (_returnvalue _height) (CallFunction|CalculateNewCapsuleLocation))
  (bind _returnvalue_2 (Components|GetOwner))
  (bind _verticaltraceheight (Variables|Settings|GetVerticalTraceHeight))
  (bind _horcolpathfromcharacter (Variables|Settings|GetHorColPathFromCharacter))
  (bind _returnvalue_3 (Transformation|GetActorLocation _returnvalue_2))
  (bind _returnvalue_4 (Transformation|GetActorForwardVector _returnvalue_2))
  (bind (_x _y _z) (Math|Vector|BreakVector _returnvalue_3))
  (bind _returnvalue_5 (* _returnvalue_4 _horcolpathfromcharacter))
  (bind _returnvalue_6 (+ _z _verticaltraceheight))
  (bind _returnvalue_7 (Math|Vector|MakeVector _x _y _returnvalue_6))
  (bind _returnvalue_8 (+ _returnvalue_7 _returnvalue_5))
  (bind (_x_2 _y_2 _z_2) (Math|Vector|BreakVector _returnvalue_8))
  (bind (_outhit _returnvalue_9) (Collision|SphereTraceByChannel _returnvalue_8 (Math|Vector|MakeVector _x_2 _y_2 (- _z_2 (Variables|Settings|GetVerticalTraceHeight))) 2e+01 "TraceTypeQuery7" false (Utilities|Array|MakeArray (Components|GetOwner)) "None"))
  (if _returnvalue_9
    (Variables|Engine|SetHeightLocation (.Location (Collision|BreakHitResult _outhit)))
    (if (CallFunction|HiptoLedge)
      (if (Variables|State|GetClimbing)
        (Variables|Engine|SetCanStartClimbing false)
        (else
          (LocalVariables|SetCapsule _returnvalue)
          (LocalVariables|SetHeight _height)
          (bind _returnvalue_10 (Collision|SphereTraceByChannel (+ (Variables|Engine|GetHeightLocation) "0.000000, 0,60.000000" (* (Transformation|GetActorForwardVector (Components|GetOwner)) -50)) (+ (+ (Variables|Engine|GetHeightLocation) "0, 0,60.000000") (* (Math|Vector|GetForwardVector (Math|Rotator|MakeRotator 0.0 0.0 (.Yaw (Math|Rotator|BreakRotator (Pawn|GetControlRotation (Variables|Engine|GetOwner) :!class /Script/Engine.Pawn))))) 5e+01)) 4e+01 "TraceTypeQuery1" false 0 "None" true "(R=0.000000,G=0.376269,B=1.000000,A=1.000000)" "(R=0.786176,G=1.000000,B=0.000000,A=1.000000)"))
          (if _returnvalue_10
            (Variables|Engine|SetCanStartClimbing false)
            (else
              (CallFunction|StartClimbing 1.8e+02 (LocalVariables|GetCapsule) (LocalVariables|GetHeight))
              (Variables|Engine|SetCanStartClimbing true))))))))

(fn HiptoLedge
  (bind _pelvissocketname (Variables|Settings|GetPelvisSocketName))
  (bind _bodymesh (CallFunction|GetCharacterSkeleton (Components|GetOwner)))
  (Utilities|IsValid (.Mesh (GetComponents|GetOwnerMesh))
    (:Is%20Valid
      (if (Transformation|DoesSocketExist _bodymesh _pelvissocketname)
        (return (Math|Float|InRange(Float) (- (.Z (Math|Vector|BreakVector (Transformation|GetSocketLocation _bodymesh _pelvissocketname))) (.Z (Math|Vector|BreakVector (Variables|Engine|GetHeightLocation)))) -1.2e+02 0.0))
        (else
          (return false))))
    (:Is%20Not%20Valid
      (return false))))

(fn GetOwnerMesh
  (bind (_defaultbodymesh _headmesh) (Class|BPIAI|GetDemoSkeletalMeshes(Message) (Components|GetOwner)))
  (return _defaultbodymesh _headmesh))

(fn GetOwnerCharacterMovement
  (return (Actor|GetComponentbyClass (Components|GetOwner) "/Script/Engine.CharacterMovementComponent")))

(fn GetOwnerCapsuleComponent
  (return (Actor|GetComponentbyClass (Components|GetOwner) "/Script/Engine.CapsuleComponent")))

(fn CalculateNewCapsuleLocation
  (bind _heightlocation (Variables|Engine|GetHeightLocation))
  (bind _collisionnormal (Variables|Engine|GetCollisionNormal))
  (bind _collisionlocation (Variables|Engine|GetCollisionLocation))
  (bind _collisionnormal_2 (Variables|Engine|GetCollisionNormal))
  (bind _collisionlocation_2 (Variables|Engine|GetCollisionLocation))
  (bind (_x _y) (Math|Vector|BreakVector _collisionlocation_2))
  (bind _z (Math|Vector|BreakVector _heightlocation))
  (bind (_x_2 _y_2) (Math|Vector|BreakVector _collisionlocation))
  (bind _returnvalue (* _collisionnormal_2 "25.000000,25.000000, 0"))
  (bind _returnvalue_2 (* _collisionnormal "25.000000,25.000000, 0"))
  (bind _returnvalue_3 (+ (.y _returnvalue) _y))
  (bind _returnvalue_4 (+ (.x _returnvalue) _x))
  (bind _returnvalue_5 (Math|Vector|MakeVector _returnvalue_4 _returnvalue_3 _z))
  (bind (_outhit _returnvalue_6) (Collision|LineTraceByChannel _returnvalue_5 (- _returnvalue_5 "0.000000,0.000000,500000.000000") "TraceTypeQuery1" false (Utilities|Array|MakeArray (Components|GetOwner)) "None"))
  (if _returnvalue_6
    (return (Math|Vector|MakeVector (+ (.x _returnvalue_2) _x_2) (+ (.y _returnvalue_2) _y_2) (- (.Z (Math|Vector|BreakVector (Variables|Engine|GetHeightLocation))) (select (> (Math|Float|Absolute(Float) (- (.Z (Math|Vector|BreakVector (.Location (Collision|BreakHitResult _outhit)))) (.Z (Math|Vector|BreakVector _returnvalue_5)))) 1.6e+02) 1.2e+02 -25.0))) (Math|Float|Absolute(Float) (- (.Z (Math|Vector|BreakVector (.Location (Collision|BreakHitResult _outhit)))) (.Z (Math|Vector|BreakVector _returnvalue_5)))))))

(fn ClimbMovement
  (params (Value :type Float%20%28double-precision%29))
  (bind _returnvalue (Components|GetOwner))
  (bind _returnvalue_2 (Transformation|GetActorLocation _returnvalue))
  (Transformation|SetActorLocation (Components|GetOwner) (Math|Interpolation|VInterpTo _returnvalue_2 (+ _returnvalue_2 (* (Transformation|GetActorRightVector _returnvalue) Value)) (Utilities|Time|GetWorldDeltaSeconds) 5.0) false false))

(fn GetAnimInstance
  (return (Components|SkeletalMesh|GetAnimInstance (.Mesh (GetComponents|GetOwnerMesh)))))

(fn GetOwnerasPawn
  (bind _aspawn (Utilities|Casting|CastToPawn (Components|GetOwner)))
  (return _aspawn))

(fn GetPlayerController
  (bind _asplayer_controller (Utilities|Casting|CastToPlayerController (Pawn|GetController (GetComponents|GetOwnerasPawn))))
  (return _asplayer_controller))

(fn CalculateLaunchVelocity
  (return (+ (* (Transformation|GetActorForwardVector (Variables|Engine|GetOwner)) 5e+02) "0, 0,500.000000")))

(fn NotClimbing
  (return (not (Variables|State|GetHanging))))

(fn GetLineTrace
  (params (Arrow :type Scene%20Component%20Object%20Reference))
  (bind _returnvalue (Transformation|GetWorldLocation Arrow))
  (return _returnvalue (+ _returnvalue (* (Math|Vector|GetForwardVector Arrow) 1e+01))))

(fn ResetRotation
  (bind _returnvalue (Components|GetOwner))
  (Transformation|SetActorRotation _returnvalue (Math|Rotator|MakeRotator 0.0 0.0 (.yaw (Transformation|GetActorRotation _returnvalue)))))

(fn CanbeClimbing
  (bind _owner (Variables|Engine|GetOwner))
  (bind _charactermovement (Variables|/Script/Engine.Character|GetCharacterMovement _owner))
  (bind _movementmode (Variables|/Script/Engine.CharacterMovementComponent|GetMovementMode _charactermovement))
  (Utilities|IsValid (Variables|Engine|GetOwner)
    (:Is%20Valid
      (return (Math|Boolean|ANDBoolean (not (Default|Aiming? (Actor|GetComponentbyClass (Variables|Engine|GetOwner) "/Game/ModernRPG/General/Blueprints/ActorComponents/Weapon/AC_Aiming.AC_Aiming_C"))) (Utilities|Enum|NotEqual(Enum) _movementmode "MOVE_Swimming") (Utilities|Enum|NotEqual(Enum) _movementmode "MOVE_Falling"))))))

(fn OnRepParkour
  (bind _ascharacter (Utilities|Casting|CastToCharacter (Components|GetOwner)))
  (bind _defaultbodymesh (Class|BPIAI|GetDemoSkeletalMeshes(Message) _ascharacter))
  (Class|BPIABP|SetIsParkour(Message) (Components|SkeletalMesh|GetAnimInstance _defaultbodymesh) (Variables|State|GetParkour)))

(fn Initialize
  (bind _ascharacter (Utilities|Casting|CastToCharacter (Components|GetOwner)))
  (Variables|Engine|SetOwner _ascharacter)
  (bind _asplayer_controller (Utilities|Casting|CastToPlayerController (Pawn|GetController (Variables|Engine|GetOwner))))
  (Variables|Engine|SetPlayerController _asplayer_controller))

(event Custom|PlayMontageReplicated
  (params (AnimMontage :type Anim%20Montage%20Object%20Reference) (InPlayRate :type Float%20%28double-precision%29) (TargetRelativeLocation :type Vector) (TargetRelativeRotation :type Rotator))
  ;[1 1 1] Play Montage
  (Networking|SwitchHasAuthority
    (:Authority
      (CallFunction|PlayMontageReplicated-ALL AnimMontage InPlayRate TargetRelativeLocation TargetRelativeRotation))
    (:Remote
      (CallFunction|PlayMontageReplicated-Server AnimMontage InPlayRate TargetRelativeLocation TargetRelativeRotation))))

(event Custom|PlayMontageReplicated%20-Server
  (params (AnimMontage :type Anim%20Montage%20Object%20Reference) (InPlayRate :type Float%20%28double-precision%29) (TargetRelativeLocation :type Vector) (TargetRelativeRotation :type Rotator))
  ;[1 1 1] Play Montage
  (CallFunction|PlayMontageReplicated-ALL AnimMontage InPlayRate TargetRelativeLocation TargetRelativeRotation))

(event Custom|PlayMontageReplicated%20-ALL
  (params (AnimMontage :type Anim%20Montage%20Object%20Reference) (InPlayRate :type Float%20%28double-precision%29) (TargetRelativeLocation :type Vector) (TargetRelativeRotation :type Rotator))
  (bind _returnvalue (GetComponents|GetOwnerCapsuleComponent))
  ;[1 1 1] Play Montage
  (Collision|SetCollisionEnabled _returnvalue "NoCollision")
  (Components|MoveComponentTo _returnvalue TargetRelativeLocation TargetRelativeRotation false false (Variables|Settings|GetInterpSpeed) true)
  (Variables|/Script/Engine.Pawn|SetbUseControllerRotationYaw (.AsCharacter (Utilities|Casting|CastToCharacter (Components|GetOwner))) false)
  (Input|DisableInput (Components|GetOwner) (Variables|Engine|GetPlayerController))
  (Utilities|MPlayAnyMontage AnimMontage InPlayRate
    (:On%20Completed
      (Default|ChangeWalkSpeed (Actor|GetComponentbyClass (Components|GetOwner) "/Game/ModernRPG/General/Blueprints/ActorComponents/SpeedChange/AC_SpeedChange.AC_SpeedChange_C") "NewEnumerator0")
      (if (not (Variables|Engine|GetWasHolstered))
        (CallFunction|ForceToggleWeapon (Components|GetOwner) false)
        (Variables|Engine|SetWasHolstered true)))
    (:On%20Notify%20Begin
      (Collision|SetCollisionEnabled (GetComponents|GetOwnerCapsuleComponent) "QueryAndPhysics")
      (Components|Movement|StopMovementImmediately (GetComponents|GetOwnerCharacterMovement))
      (Input|EnableInput (Variables|Engine|GetOwner) (GetComponents|GetPlayerController))
      (Variables|/Script/Engine.Pawn|SetbUseControllerRotationYaw (.AsCharacter (Utilities|Casting|CastToCharacter (Components|GetOwner))) true)
      (CallFunction|StopClimbing)
      (bind _output_get (Variables|State|SetParkour false))
      (CallFunction|ReplicateJumping _output_get))))