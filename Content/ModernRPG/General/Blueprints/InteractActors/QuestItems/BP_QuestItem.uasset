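; Quest item pickup actor that goes into the interacting character's inventory and updates their quest, with a widget shown while marked.
; CanInteract checks by item type: weapons, armor and bags test equipment slots before falling back to inventory space, other types test space directly.
; Interact confirms the character has the linked quest, adds the item, calls SetNewQuestInActor on the quest handler, then replicates destruction by authority or server call.
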(event Custom|ReplicateInventory
  (params (RememberInventory :type AC%20Inventory%20Object%20Reference))
  (Variables|Default|SetRememberInventory RememberInventory))

(event EventMarkArea
  (params (Owner :type Actor%20Object%20Reference))
  (Rendering|SetVisibility (Variables|Default|GetWidget) true false))

(event EventUnmarkArea
  (Rendering|SetVisibility (Variables|Default|GetWidget) false false))

(event EventInteract-Server
  (params (InputPin :type Character%20Object%20Reference)))

(event EventInteract
  (params (Character :type Character%20Object%20Reference))
  (bind _output_get (Variables|Default|SetInteractedCharacter Character))
  (Actor|SetOwner _output_get)
  (bind (_result _inventory) (CallFunction|CanInteract (Variables|Default|GetInteractedCharacter)))
  (if _result
    (bind _output_get_2 (Variables|Default|SetRememberInventory (Variables|/Game/ModernRPG/General/GUI/Widgets/Inventory/WB_Inventory.WB_Inventory_C|GetCurrentInventory _inventory)))
    (CallFunction|ReplicateInventory _output_get_2)
    (Variables|Default|SetCurrentActor (Variables|Default|GetInteractedCharacter))
    (bind _outputpin (Default|FindQuest (Actor|GetComponentbyClass (Variables|Default|GetCurrentActor) "/Game/ModernRPG/General/Blueprints/DialoguesQuests/MapComponents/AC_QuestsHandler.AC_QuestsHandler_C") (.Quest (Utilities|Struct|BreakS_QuestDynam (Variables|/Game/ModernRPG/General/Blueprints/DialoguesQuests/Quests/AC_QuestActor.AC_QuestActor_C|GetCurrentQuest (Variables|Default|GetAC_QuestActor))))))
    (if (!= _outputpin -1)
      (Utilities|IsValid (.DataTable (Utilities|Struct|BreakDataTableRowHandle (.Row (Utilities|Struct|BreakS_InvItemDyn (Variables|Default|GetQuestItem)))))
        (:Is%20Valid
          (bind (_result_2 _inventory_2 _location _selectedslots) (Default|CanAddtoInventory (Variables|Default|GetRememberInventory) (.Size (Utilities|Struct|BreakS_InventorySlot (.InvTexture (Utilities|Struct|BreakS_InventoryItem (CallFunction|GetItemInfo (.Row (Utilities|Struct|BreakS_InvItemDyn (Variables|Default|GetQuestItem)))))))) (Variables|Default|GetQuestItem)))
          (if _result_2
            (Utilities|IsValid (Variables|/Game/ModernRPG/General/Blueprints/ActorComponents/Character/Inventory/AC_Inventory.AC_Inventory_C|GetInventoryWidget (Variables|/Game/ModernRPG/General/GUI/Widgets/Inventory/WB_Inventory.WB_Inventory_C|GetCurrentInventory _inventory_2))
              (:Is%20Valid
                (Default|AddItem (Variables|/Game/ModernRPG/General/GUI/Widgets/Inventory/WB_Inventory.WB_Inventory_C|GetCurrentInventory _inventory_2) (Variables|Default|GetQuestItem) (Variables|Default|GetCurrentActor) _location _selectedslots (Variables|/Game/ModernRPG/General/Blueprints/ActorComponents/Character/Inventory/AC_Inventory.AC_Inventory_C|GetInventoryWidget (Variables|/Game/ModernRPG/General/GUI/Widgets/Inventory/WB_Inventory.WB_Inventory_C|GetCurrentInventory _inventory_2))))
              (:Is%20Not%20Valid
                _))
            (Default|SetNewQuestinActor (Actor|GetComponentbyClass (Variables|Default|GetCurrentActor) "/Game/ModernRPG/General/Blueprints/DialoguesQuests/MapComponents/AC_QuestsHandler.AC_QuestsHandler_C") (Variables|Default|GetQuestActor) (Variables|Default|GetDialoguePart) self)
            (Networking|SwitchHasAuthority
              (:Authority
                (CallFunction|ReplicateDestroy true))
              (:Remote
                (CallFunction|ReplicateDestroy-Server true)))))))))

(fn ConstructionScript
  (|CallParentFunction))

(fn CanInteract
  (params (Character :type Actor%20Object%20Reference))
  (switch Utilities|FlowControl|Switch|SwitchonE_ItemType (.Type (Utilities|Struct|BreakS_InventoryItem (CallFunction|GetItemInfo (.Row (Utilities|Struct|BreakS_InvItemDyn (Variables|Default|GetQuestItem))))))
    (:NewEnumerator0
      (if (Default|CantAddtoComponent? (Actor|GetComponentbyClass Character "/Game/ModernRPG/General/Blueprints/ActorComponents/InteractActors/AC_EquipmentHandler.AC_EquipmentHandler_C") (Variables|Default|GetQuestItem))
        _
        (else
          (return true 0))))
    (:NewEnumerator1
      (if (.Result (Default|HasSameArmorType? (Actor|GetComponentbyClass Character "/Game/ModernRPG/General/Blueprints/ActorComponents/Weapon/AC_ArmorEquipment.AC_ArmorEquipment_C") (Variables|Default|GetQuestItem)))
        _
        (else
          (return true 0))))
    (:NewEnumerator2
      (bind (_result _inventory) (Default|CanAddtoInventory (Actor|GetComponentbyClass Character "/Game/ModernRPG/General/Blueprints/ActorComponents/Character/Inventory/AC_Inventory.AC_Inventory_C") (.Size (Utilities|Struct|BreakS_InventorySlot (.InvTexture (Utilities|Struct|BreakS_InventoryItem (CallFunction|GetItemInfo (.Row (Utilities|Struct|BreakS_InvItemDyn (Variables|Default|GetQuestItem)))))))) (Variables|Default|GetQuestItem) :!label _label))
      (return _result _inventory))
    (:NewEnumerator3
      (goto _label))
    (:NewEnumerator4
      (goto _label))
    (:NewEnumerator5
      (goto _label))
    (:NewEnumerator6
      (goto _label))
    (:NewEnumerator7
      (if (.Result (Default|HasSameBagType? (Actor|GetComponentbyClass Character "/Game/ModernRPG/General/Blueprints/ActorComponents/Weapon/AC_ArmorEquipment.AC_ArmorEquipment_C") (Variables|Default|GetQuestItem)))
        _
        (else
          (return true 0))))
    (:NewEnumerator9
      (goto _label)))
  (bind (_result_2 _inventory_2) (Default|CanAddtoInventory (Actor|GetComponentbyClass Character "/Game/ModernRPG/General/Blueprints/ActorComponents/Character/Inventory/AC_Inventory.AC_Inventory_C") (.Size (Utilities|Struct|BreakS_InventorySlot (.InvTexture (Utilities|Struct|BreakS_InventoryItem (CallFunction|GetItemInfo (.Row (Utilities|Struct|BreakS_InvItemDyn (Variables|Default|GetQuestItem)))))))) (Variables|Default|GetQuestItem)))
  (return _result_2 _inventory_2))