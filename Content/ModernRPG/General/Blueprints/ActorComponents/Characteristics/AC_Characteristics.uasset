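; Actor component for one character stat (Health, Stamina, Food or Water), with modifiers, skill-tree bonuses and save/load.
; Looping timers drive delayed regeneration and periodic spending, with stamina draining only while moving.
; Changes set a clamped NewVal replicated through server and multicast events, whose OnRep enables a gated Tick that eases CurVal toward it.
; Tick broadcasts value changes, throttles CurVal replication and updates an optional widget.
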(event Custom|OnModifierAdded
  (params (Type :type E_StatType%20Enum :default "NewEnumerator0") (Value :type Float%20%28double-precision%29))
  ;[1 1 1] Manipulate Modification
  (if (Utilities|Enum|Equal(Enum) Type (Variables|StatType|GetType))
    (Modifier|AddModifier Value)))

(event Custom|OnModifierRemoved
  (params (Type :type E_StatType%20Enum :default "NewEnumerator0") (Value :type Float%20%28double-precision%29))
  ;[1 1 1] Manipulate Modification
  (if (Utilities|Enum|Equal(Enum) Type (Variables|StatType|GetType))
    (Modifier|RemoveModifier Value)))

(event Custom|ReplicateValue
  (bind _curval (Variables|State|GetCurVal))
  ;[1 1 1] Replicate Value
  (if (Variables|Default|GetShouldReplicate)
    (if (Variables|Default|GetCanReplicate?)
      (Variables|Default|SetCanReplicate? false)
      (Utilities|FlowControl|Sequence
        (:then_0
          (if (Ability|HasAuthority (Components|GetOwner))
            (CallFunction|SetValue-ALL _curval)
            (else
              (CallFunction|SetValue-Server _curval))))
        (:then_1
          (Utilities|FlowControl|Delay 1.0)
          (Variables|Default|SetCanReplicate? true))))))

(event Custom|SetValue%20-ALL
  (params (CurVal :type Float%20%28double-precision%29))
  ;[1 1 1] Replicate Widget Value
  (Variables|State|SetCurVal CurVal))

(event Custom|SpentEvent
  ;[1 1 1] Spent Event
  (if (Variables|Default|GetCanSpent)
    (if (Utilities|Enum|Equal(Enum) (Variables|StatType|GetType) "NewEnumerator2")
      (if (> (Math|Vector|VectorLength (Transformation|GetVelocity (Components|GetOwner))) 0.0)
        (Statistic|ModifyStat (* (Variables|Spent|GetSpentValue) -1.0) true :!label _label))
      (else
        (goto _label)))))

(event Custom|BindSpentEvent
  ;[1 1 1] Spent Event Process
  (bind _aspawn (Utilities|Casting|CastToPawn (Components|GetOwner)))
  (if (Pawn|IsLocallyControlled _aspawn)
    (CallFunction|SpentEvent)))

(event Custom|StopSpentEvent
  ;[1 1 1] Stop spent event
  (CallFunction|StopSpentEvent-OC))

(event Custom|ForceUpdate
  (params (NewValue :type Float%20%28double-precision%29))
  ;[1 1 1] Update The Value
  (Default|CallOnValueChanged NewValue (Variables|State|GetMax)))

(event Custom|SetCanSpent%20-Server
  (params (CanSpent :type Boolean))
  ;[1 1 1] Can stop spent
  (CallFunction|SetCanSpent-ALL CanSpent))

(event Custom|SetCanSpent%20-ALL
  (params (CanSpent :type Boolean))
  ;[1 1 1] Can stop spent
  (Variables|Default|SetCanSpent CanSpent))

(event Custom|ClearTimer
  ;[1 1 1] Replicate Cleared Timer
  (if (Ability|HasAuthority (Components|GetOwner))
    (CallFunction|ClearTimer-ALL)
    (else
      (CallFunction|ClearTimer-Server))))

(event Custom|SetValue%20-Server
  (params (CurVal :type Float%20%28double-precision%29))
  ;[1 1 1] Replicate Widget Value
  (CallFunction|SetValue-ALL CurVal))

(event Custom|UpdateDamageLocation%20-Server
  (params (Location :type Vector))
  ;[1 1 1] Update Damage Location
  (CallFunction|UpdateDamageLocation-OC Location))

(event Custom|ClearTimer%20-Server
  ;[1 1 1] Replicate Cleared Timer
  (CallFunction|ClearTimer-ALL))

(event Custom|ClearTimer%20-ALL
  ;[1 1 1] Replicate Cleared Timer
  (Utilities|Time|ClearandInvalidateTimerbyHandle (Variables|Regenerate|GetTimer)))

(event Custom|ReplicateNewValue
  (bind _newval (Variables|State|GetNewVal))
  ;[1 1 1] Replicate New Value
  (if (Ability|HasAuthority (Components|GetOwner))
    (CallFunction|ReplicateNewValue-ALL _newval)
    (else
      (CallFunction|ReplicateNewValue-Server _newval))))

(event Custom|ReplicateNewValue%20-Server
  (params (NewVal :type Float%20%28double-precision%29))
  ;[1 1 1] Replicate New Value
  (CallFunction|ReplicateNewValue-ALL NewVal))

(event Custom|ReplicateNewValue%20-ALL
  (params (NewVal :type Float%20%28double-precision%29))
  ;[1 1 1] Replicate New Value
  (Variables|State|SetNewVal NewVal))

(event Custom|ChangeMaxValue_Skill
  (params (Stat :type E_StatType%20Enum :default "NewEnumerator1"))
  ;[1 1 1] Apply Skills
  (if (Utilities|Enum|Equal(Enum) Stat (Variables|StatType|GetType))
    (bind _output_get (Variables|State|SetMax (Statistic|GetMaxValueSkill)))
    (bind _output_get_2 (Variables|State|SetCurVal _output_get))
    (Variables|State|SetNewVal _output_get_2)
    (CallFunction|ReplicateNewValue)
    (Default|CallOnValueChanged (Variables|State|GetCurVal) (Variables|State|GetCurVal))))

(event Custom|StartAnimation
  ;[1 1 1] Toggle Event Tick
  (Components|Tick|SetComponentTickEnabled true)
  (Utilities|FlowControl|Gate true) ; enters at Open
)

(event Custom|StopAnimation
  ;[1 1 1] Toggle Event Tick
  (Components|Tick|SetComponentTickEnabled false)
  (Utilities|FlowControl|Gate true) ; enters at Close
)

(event Custom|SpentEvent%20-Server
  ;[1 1 1] Spent Event
  (CallFunction|SpentEvent))

(event Custom|SpentEvent
  ;[1 1 1] Spent Event
  (Utilities|FlowControl|DoOnce false
    (:Completed
      (bind _returnvalue (Utilities|Time|SetTimerbyEvent (delegate Custom|SpentEvent) (Variables|Spent|GetSpentRate) true))
      (Variables|Default|SetSpentTimer _returnvalue))))

(event Custom|SetMaxValue
  ;[1 1 1] Reset Characteristic
  (Statistic|SetCurrentValue (Variables|State|GetMax) false)
  (bind _output_get (Variables|State|SetCurVal (Variables|State|GetMax)))
  (Default|CallOnValueChanged _output_get (Statistic|GetMaxValue))
  (CallFunction|ReplicateValue)
  (if (Variables|Widget|GetNeedWidget)
    (CallFunction|SetWidgetValue (Math|Float|MapRangeClamped (Variables|State|GetCurVal) (Variables|State|GetMax) 0.0 0.0 1.0))))

(event Custom|ResetDO
  ;[1 1 1] Spent Event
  (Utilities|FlowControl|DoOnce false) ; enters at Reset
)

(event Custom|StopSpentEvent%20-OC
  ;[1 1 1] Stop spent event
  (Utilities|Time|PauseTimerbyHandle (Variables|Default|GetSpentTimer))
  (CallFunction|ResetDO))

(event Custom|OnBaseValueChanged
  (params (Stat :type E_StatType%20Enum :default "NewEnumerator0") (NewValue :type Float%20%28double-precision%29))
  ;[1 1 1] Change Max Value
  (if (Utilities|Enum|Equal(Enum) Stat (Variables|StatType|GetType))
    (Variables|State|SetMax NewValue)
    (Default|CallOnValueChanged (Variables|State|GetCurVal) (Statistic|GetMaxValue))))

(event Custom|CreateWidget%20-Server
  ;[1 1 1] Create Damage Widget
  (CallFunction|CreateWidget-OC))

(event Custom|UpdateRegeneration
  ;[1 1 1] Regeneration Update
  (if (and (Variables|Regenerate|GetCanRegenerate) (not (Utilities|Time|IsTimerActivebyHandle (Variables|Regenerate|GetTimer))))
    (Utilities|FlowControl|RetriggerableDelay (Variables|Regenerate|GetRegenDelay))
    (CallFunction|StartRegenerating)))

(event Custom|StartRegenerating
  ;[1 1 1] Regeneration
  (bind _returnvalue (Utilities|Time|SetTimerbyFunctionName 0 "RegenTick" (CallFunction|GetRegenerationTickInterval) true))
  (Variables|Regenerate|SetTimer _returnvalue))

(event Custom|CreateWidget%20-OC
  ;[1 1 1] Create Damage Widget
  (bind _returnvalue (UserInterface|CreateWidget (Variables|Widget|GetWidget)))
  (Utilities|IsValid _returnvalue
    (:Is%20Valid
      (UserInterface|Viewport|AddtoViewport _returnvalue 0)
      (Variables|Default|SetDamage _returnvalue))))

(event Custom|UpdateDamageLocation%20-OC
  (params (Location :type Vector))
  ;[1 1 1] Update Damage Location
  (Class|BPIWidgetsInfo|UpdateDamageLocation(Message) (Variables|Default|GetDamage) Location))

(event Custom|BlockCharacteristic
  ;[1 1 1] Reset Characteristic
  (Statistic|SetCurrentValue 0.0 false)
  (Utilities|Time|PauseTimerbyHandle (Variables|Regenerate|GetTimer))
  (Regeneration|ClearRegenTimer))

(event Custom|SetWidgetValue
  (params (Value :type Float%20%28double-precision%29))
  ;[1 1 1] Replicate Widget Value
  (Class|BPIWidgetsInfo|SetValue(Message) (Variables|Default|GetDamage) Value))

(event EventTick
  (params (DeltaSeconds :type Float%20%28single-precision%29))
  ;[1 1 1] Toggle Event Tick
  (Utilities|FlowControl|Gate true
    (:Exit
      ;[1 1 1] Go to the new value softly
      (if (!= (Variables|State|GetCurVal) (Variables|State|GetNewVal))
        (if (CallFunction|ControlChangableValue)
          (Variables|State|SetCurVal (Math|Interpolation|FInterpTo (Variables|State|GetCurVal) (Variables|State|GetNewVal) (Utilities|Time|GetWorldDeltaSeconds) 1e+01))
          (Default|CallOnValueChanged (Variables|State|GetCurVal) (Variables|State|GetMax))
          (CallFunction|ReplicateValue)
          (if (Variables|Widget|GetNeedWidget)
            (CallFunction|SetWidgetValue (Math|Float|MapRangeClamped (Variables|State|GetCurVal) (Variables|State|GetMax) 0.0 0.0 1.0))))
        (else
          (CallFunction|StopAnimation))))))

(event EventBeginPlay
  ;[1 1 1] Set Values
  (Variables|Regenerate|SetInitialRegenValue (Variables|Regenerate|GetRegenValue))
  (if (Variables|Spent|GetSpentable)
    (CallFunction|BindSpentEvent))
  (CallFunction|UpdateRegeneration)
  (Utilities|FlowControl|Sequence
    (:then_0
      (if (Variables|Widget|GetNeedWidget)
        (CallFunction|CreateWidget-Server)))
    (:then_1
      (Utilities|FlowControl|Delay 2.5)
      (bind _hassave (Save|LoadStat))
      (if (not _hassave)
        (Statistic|SetCurrentValue (Variables|State|GetMax) false)
        (Utilities|FlowControl|Delay 0.2)
        (CallFunction|SetWidgetValue 0.0)))))

(fn ModifyStat
  (params (Value :type Float%20%28double-precision%29) (InterruptRegeneration :type Boolean))
  (bind _curval (Variables|State|GetCurVal))
  (bind _returnvalue (+ _curval Value))
  (if (!= Value 0.0)
    (if InterruptRegeneration
      (Regeneration|ClearRegenTimer))
    (Statistic|SetCurrentValue (Math|Float|SelectFloat (Math|Float|SelectFloat 0.0 _returnvalue (<= _returnvalue 0.0)) _returnvalue (Variables|StatType|GetClampZero)) false)
    (CallFunction|UpdateRegeneration)
    (if (<= (+ (Variables|State|GetCurVal) Value) 0.05)
      (Default|CallBelowZero (Variables|Spent|GetSpentDamage)))))

(fn RegenTick
  (bind _regenvalue (Variables|Regenerate|GetRegenValue))
  (if (< (Variables|State|GetCurVal) (Statistic|GetMaxValue))
    (Statistic|ModifyStat (+ (* (/ (CallFunction|GetModifierPerk) 1e+02) _regenvalue) _regenvalue) false)
    (else
      (Regeneration|ClearRegenTimer))))

(fn ClearRegenTimer
  (Utilities|Time|ClearandInvalidateTimerbyHandle (Variables|Regenerate|GetTimer))
  (CallFunction|ClearTimer))

(fn GetMaxValue
  (switch Utilities|FlowControl|Switch|SwitchonE_StatType (Variables|StatType|GetType)
    (:NewEnumerator1
      (return (+ (Variables|State|GetMax) (Variables|ExtendedStat|GetModifierValue))))
    (:NewEnumerator2
      (return (+ (Variables|State|GetMax) (Variables|ExtendedStat|GetModifierValue))))
    (:NewEnumerator3
      _)
    (:NewEnumerator15
      _))
  (return (+ (Variables|State|GetMax) (Variables|ExtendedStat|GetModifierValue))))

(fn AddModifier
  (params (Value :type Float%20%28double-precision%29))
  (Variables|ExtendedStat|SetModifierValue (+ Value (Variables|ExtendedStat|GetModifierValue))))

(fn RemoveModifier
  (params (Value :type Float%20%28double-precision%29))
  (Variables|ExtendedStat|SetModifierValue (- (Variables|ExtendedStat|GetModifierValue) Value))
  (Statistic|SetCurrentValue (Math|Float|Clamp(Float) (Variables|State|GetCurVal) 0.0 (Statistic|GetMaxValue)) false)
  (CallFunction|UpdateRegeneration))

(fn SetCurrentValue
  (params (Value :type Float%20%28double-precision%29) (InterruptRegeneration :type Boolean))
  (Variables|State|SetNewVal (Math|Float|Clamp(Float) Value -1e+02 (Statistic|GetMaxValue)))
  (CallFunction|ReplicateNewValue)
  (if InterruptRegeneration
    (Regeneration|ClearRegenTimer)
    (CallFunction|UpdateRegeneration)))

(fn SaveStat
  (bind _returnvalue (SaveGame|DoesSaveGameExist (Save|GetSlotName)))
  (if _returnvalue
    (bind _returnvalue_2 (SaveGame|LoadGamefromSlot (Save|GetSlotName)))
    (bind _asbp_save_characteristics (Utilities|Casting|CastToBP_SaveCharacteristics _returnvalue_2))
    (LocalVariables|SetL_GameSave _asbp_save_characteristics)
    (else
      (bind _returnvalue_3 (SaveGame|CreateSaveGameObject "/Game/ModernRPG/General/Blueprints/Characteristics/BP_SaveCharacteristics.BP_SaveCharacteristics_C"))
      (LocalVariables|SetL_GameSave _returnvalue_3)))
  (Variables|/Game/ModernRPG/General/Blueprints/Characteristics/BP_SaveCharacteristics.BP_SaveCharacteristics_C|SetsNewValue (LocalVariables|GetL_GameSave) (Variables|State|GetNewVal))
  (SaveGame|SaveGametoSlot (LocalVariables|GetL_GameSave) (Save|GetSlotName)))

(fn LoadStat
  (bind _returnvalue (SaveGame|DoesSaveGameExist (Save|GetSlotName)))
  (if _returnvalue
    (bind _returnvalue_2 (SaveGame|LoadGamefromSlot (Save|GetSlotName)))
    (bind _asbp_save_characteristics (Utilities|Casting|CastToBP_SaveCharacteristics _returnvalue_2))
    (bind _output_get (LocalVariables|SetL_GameSave _asbp_save_characteristics))
    (Statistic|SetCurrentValue (Variables|/Game/ModernRPG/General/Blueprints/Characteristics/BP_SaveCharacteristics.BP_SaveCharacteristics_C|GetsNewValue _output_get) true)
    (return true)
    (else
      (return false))))

(fn GetSlotName
  (return (Utilities|String|Append (Variables|Save|GetStatSlot) "_" (Variables|Save|GetAddSlotName))))

(fn SetCanSpent
  (params (CanSpent :type Boolean))
  (CallFunction|SetCanSpent-Server CanSpent))

(fn DebugCharacteristic
  (bind _aspawn (Utilities|Casting|CastToPawn (Components|GetOwner)))
  (if (Pawn|IsPlayerControlled _aspawn)
    (Development|PrintString (Utilities|String|Append (Utilities|String|EnumtoString (Variables|StatType|GetType)) "  " (Utilities|String|ToString(Float) (Variables|State|GetCurVal))) true true "(R=0.000000,G=0.660000,B=1.000000,A=1.000000)" 0.0)))

(fn GetModifierPerk
  (bind _returnvalue (Components|GetOwner))
  (bind _returnvalue_2 (Actor|GetComponentbyClass _returnvalue "/Game/ModernRPG/ModernSkillTree/ActorComponent/AC_SkillTree.AC_SkillTree_C"))
  (return (Utilities|Select :Index (Variables|StatType|GetType) :NewEnumerator1 (Variables|/Game/ModernRPG/ModernSkillTree/ActorComponent/AC_SkillTree.AC_SkillTree_C|GetHealthRegenerationModifier _returnvalue_2) :NewEnumerator2 (Variables|/Game/ModernRPG/ModernSkillTree/ActorComponent/AC_SkillTree.AC_SkillTree_C|GetEnduranceModifier _returnvalue_2) :NewEnumerator3 1.0 :NewEnumerator15 1.0)))

(fn GetRegenerationTickInterval
  (return (Variables|ExtendedStat|GetRegenerationTickInterval)))

(fn GetMaxValueSkill
  (bind _returnvalue (Components|GetOwner))
  (bind _returnvalue_2 (Actor|GetComponentbyClass _returnvalue "/Game/ModernRPG/ModernSkillTree/ActorComponent/AC_SkillTree.AC_SkillTree_C"))
  (switch Utilities|FlowControl|Switch|SwitchonE_StatType (Variables|StatType|GetType)
    (:NewEnumerator1
      (return (* (+ (/ (Variables|/Game/ModernRPG/ModernSkillTree/ActorComponent/AC_SkillTree.AC_SkillTree_C|GetHealthModifier _returnvalue_2) 1e+02) 1.0) (+ (Variables|State|GetMax) (Variables|ExtendedStat|GetModifierValue)))))
    (:NewEnumerator2
      (return (* (+ (/ (Variables|/Game/ModernRPG/ModernSkillTree/ActorComponent/AC_SkillTree.AC_SkillTree_C|GetEnduranceModifier _returnvalue_2) 1e+02) 1.0) (+ (Variables|State|GetMax) (Variables|ExtendedStat|GetModifierValue)))))
    (:NewEnumerator3
      _)
    (:NewEnumerator15
      _))
  (return (+ (Variables|State|GetMax) (Variables|ExtendedStat|GetModifierValue))))

(fn ControlChangableValue
  (if (Utilities|Enum|Equal(Enum) (Variables|StatType|GetType) "NewEnumerator2")
    (if (Variables|/Game/ModernRPG/ModernSkillTree/ActorComponent/AC_SkillTree.AC_SkillTree_C|GetSprintUnlimit (Actor|GetComponentbyClass (Components|GetOwner) "/Game/ModernRPG/ModernSkillTree/ActorComponent/AC_SkillTree.AC_SkillTree_C"))
      (return false)
      (else
        (return true)))
    (else
      (return true))))

(fn HasEnergy
  (params (Value :type Float%20%28double-precision%29))
  (return (>= (- (Variables|State|GetCurVal) Value) 0.0)))

(fn OnRepNewVal
  (CallFunction|StartAnimation))