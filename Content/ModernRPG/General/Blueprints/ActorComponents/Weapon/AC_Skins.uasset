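; Actor component that applies the current modular skin to its owning Character's head, body, torso, legs and feet meshes.
; On BeginPlay, the locally controlled player waits three seconds, then applies any non-default skin.
; The request goes through Server and ALL events by authority, so the change is networked.
; A loop pairs skin parts to mesh components by index, swapping each mesh, anim class and materials.
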(event Custom|ApplySkinsToAllMeshComponents
  ;[1 1 1] Initialize Mesh Information
  (bind (_head _body _torso _legs _feet _animbp) (CallFunction|GetCurrentSkin))
  (Networking|SwitchHasAuthority
    (:Authority
      (CallFunction|ApplySkinstoAllMeshComponents-ALL (Utilities|Array|MakeArray _head _body _torso _legs _feet) _animbp))
    (:Remote
      (CallFunction|ApplySkinstoAllMeshComponents-Server (Utilities|Array|MakeArray _head _body _torso _legs _feet) _animbp))))

(event Custom|ApplySkinsToAllMeshComponents%20-%20ALL
  (params (Skins :type Array%20of%20S%20Character%20Skin%20Separated%20Structures) (Anim :type Anim%20Instance%20Class%20Reference))
  ;[1 1 1] Initialize Mesh Information
  (CallFunction|ApplySkinstoAllMeshComponents-Loop Skins Anim))

(event Custom|ApplySkinsToAllMeshComponents%20-%20Server
  (params (Skins :type Array%20of%20S%20Character%20Skin%20Separated%20Structures) (Anim :type Anim%20Instance%20Class%20Reference))
  ;[1 1 1] Initialize Mesh Information
  (CallFunction|ApplySkinstoAllMeshComponents-ALL Skins Anim))

(event EventBeginPlay
  ;[1 1 1] Initialize Skins
  (bind _ascharacter (Utilities|Casting|CastToCharacter (Components|GetOwner)))
  (bind _output_get (Variables|Default|SetPlayer _ascharacter))
  (if (Pawn|IsLocallyControlled _output_get)
    (Utilities|FlowControl|Delay 3.0)
    (bind _default (CallFunction|GetCurrentSkin))
    (if (not _default)
      (CallFunction|ApplySkinstoAllMeshComponents))))

(fn InitializeNewSkin)

(fn ApplyNewBodyPartNewMaterials
  (params (CurrentBodyPart%28instance%29 :type Skeletal%20Mesh%20Component%20Object%20Reference) (NewBodyPart :type Skeletal%20Mesh%20Object%20Reference) (NewMaterials :type Array%20of%20Material%20Instance%20Object%20References) (NewAnimClass :type Object%20Class%20Reference))
  (Components|SkinnedMesh|SetSkinnedAssetandUpdate CurrentBodyPart%28instance%29 NewBodyPart true)
  (Class|SkeletalMeshComponent|SetAnimClass CurrentBodyPart%28instance%29 NewAnimClass)
  (for (_array_element _array_index) NewMaterials
    (Rendering|Material|SetMaterial CurrentBodyPart%28instance%29 _array_index _array_element))
  (return))

(fn ApplySkinstoAllMeshComponents-Loop
  (params (Skins :type Array%20of%20S%20Character%20Skin%20Separated%20Structures) (Anim :type Anim%20Instance%20Class%20Reference))
  (LocalVariables|SettempArray Skins)
  (LocalVariables|SettempAnimBP Anim)
  (bind (_headmesh _bodymesh _torsomesh _legsmesh _feetmesh) (CallFunction|GetCharacterSkeleton (Variables|Default|GetPlayer)))
  (for (_array_element _array_index) (Utilities|Array|MakeArray _headmesh _bodymesh _torsomesh _legsmesh _feetmesh)
    (Utilities|IsValid _array_element
      (:Is%20Valid
        (CallFunction|ApplyNewBodyPartNewMaterials _array_element (.SkeletalMesh (Utilities|Struct|BreakS_CharacterSkin_Separated (Utilities|Array|Get(acopy) (LocalVariables|GettempArray) _array_index))) (.Materials (Utilities|Struct|BreakS_CharacterSkin_Separated (Utilities|Array|Get(acopy) (LocalVariables|GettempArray) _array_index))) (LocalVariables|GettempAnimBP)))))
  (return))