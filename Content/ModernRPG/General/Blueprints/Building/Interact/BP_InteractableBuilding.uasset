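; BP_InteractableBuilding is a building Blueprint that hosts an interact actor through a child actor component.
; On BeginPlay it takes ownership of the child, casts it to BP_InteractActor and hands it a back-reference to the building.
; Start activates the particle system and sends a start message to the child.
; ControlCollision forwards collision changes to the child by message.
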(event Custom|SetupBP_Building
  (params (InteractActor :type BP%20Interact%20Actor%20Object%20Reference) (BP_Building :type Actor%20Object%20Reference))
  (Variables|/Game/ModernRPG/General/Blueprints/InteractActors/BP_InteractActor.BP_InteractActor_C|SetBP_Building InteractActor BP_Building))

(event EventBeginPlay
  (bind _childactor (Variables|Default|GetChildActor))
  (bind _childactor_2 (Variables|/Script/Engine.ChildActorComponent|GetChildActor _childactor))
  (|CallParentFunction)
  (Actor|SetOwner _childactor_2 self)
  (bind _asbp_interact_actor (Utilities|Casting|CastToBP_InteractActor _childactor_2))
  (CallFunction|SetupBPBuilding _asbp_interact_actor self))

(event Collision|EventActorBeginOverlap
  (params (OtherActor :type Actor%20Object%20Reference))
  (|CallParentFunction OtherActor) ; This node is disabled and will not be called.\nDrag off pins to build functionality.
)

(event EventTick
  (params (DeltaSeconds :type Float%20%28single-precision%29))
  (|CallParentFunction DeltaSeconds))

(event EventStart
  (Components|Activation|Activate (Variables|Default|GetParticleSystem) false)
  (Class|BPIBuilding|Start(Message) (Variables|/Script/Engine.ChildActorComponent|GetChildActor (Variables|Default|GetChildActor))))

(event EventControlCollision
  (params (collision%20enabled :type ECollisionEnabled%20Enum :default "NoCollision"))
  (Class|BPIInteract|ControlCollision(Message) (Variables|/Script/Engine.ChildActorComponent|GetChildActor (Variables|Default|GetChildActor)) collision%20enabled))

(fn ConstructionScript
  (|CallParentFunction))