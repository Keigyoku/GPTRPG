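; BP_BuldingsSaveController restores saved buildings when play begins, on the authority only.
; It loads the BP_SaveBuilding save from the BuildingSlot, if one exists, and passes each stored record to ServerLoadBuildings.
; That event spawns the saved class at its transform flagged as pregenerated, ignoring collision, then reapplies its mesh fix location and health.
; The graph only loads; it writes no saves.
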(event Custom|ServerLoadBuildings
  (params (Building :type S%20Save%20Building%20Structure))
  (bind _returnvalue (Game|SpawnActorfromClass (.class Building) (.actortransform Building) "AlwaysSpawn" 0 0 false true 0))
  (Default|ControlFixLocation-ALL _returnvalue (.staticmeshfixlocation Building))
  (Default|SetCurrentHealth-All _returnvalue (.health Building) (Variables|/Game/ModernRPG/General/Blueprints/Building/Master/BP_BuildingsMaster.BP_BuildingsMaster_C|GetMaxHealth _returnvalue)))

(event EventBeginPlay
  (Networking|SwitchHasAuthority
    (:Authority
      (bind _returnvalue (SaveGame|DoesSaveGameExist (Variables|Default|GetBuildingSlot)))
      (if _returnvalue
        (bind _returnvalue_2 (SaveGame|LoadGamefromSlot (Variables|Default|GetBuildingSlot)))
        (bind _asbp_save_building (Utilities|Casting|CastToBP_SaveBuilding _returnvalue_2))
        (for _array_element (Variables|/Game/ModernRPG/General/Blueprints/Building/Save/BP_SaveBuilding.BP_SaveBuilding_C|GetsBuildings _asbp_save_building)
          (CallFunction|ServerLoadBuildings _array_element))))))

(fn ConstructionScript)