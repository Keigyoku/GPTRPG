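; Base interactable actor for placeable buildings, configured from a data table row, covering placement, health and upgrade interaction.
; In build mode, Tick gets server-replicated validity from ground, pawn, building and BP_CollisionBuilding socket overlaps, tinting materials accordingly.
; Building restores materials, enables collision and child sockets, and disables its socket until destruction.
; Damage briefly shows a health widget and destroys at zero; interaction requests upgrades through AC_Building.
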(event Custom|BuildBuilding%20-%20Server
  (params (CollisionBuilding :type BP%20Collision%20Building%20Object%20Reference))
  ;[0 0 0] Build Object
  (if (Variables|Engine|GetCanBuild)
    (bind _output_get (Variables|Components|SetCollisionBuilding CollisionBuilding))
    (CallFunction|BuildObject-All _output_get)))

(event Custom|SetupWidget
  ;[0 0 0] Upgrade buildings - FUTURE UPDATE
  (bind _aswb_upgrade_building (Utilities|Casting|CastToWB_UpgradeBuilding (UserInterface|GetUserWidgetObject (Variables|Default|GetRadiusWidget))))
  (Variables|/Game/ModernRPG/General/GUI/Widgets/Interactions/WB_UpgradeBuilding.WB_UpgradeBuilding_C|SetBuilding _aswb_upgrade_building self))

(event Custom|ControlFixLocation%20-%20ALL
  (params (NewLocation :type Vector))
  ;[0 0 0] Build Object
  (Transformation|SetRelativeLocation (Variables|Default|GetStaticMesh) NewLocation false true))

(event Custom|ReplicateCanBuild
  (params (CanBuild :type Boolean))
  ;[0 0 0] Can Build - Event Tick
  (CallFunction|ReplicateCanBuild-All CanBuild))

(event Custom|CustomEvent
  (params (DestroyedActor :type Actor%20Object%20Reference))
  (Utilities|IsValid (Variables|Components|GetCollisionBuilding)
    (:Is%20Valid
      (Default|ControlCollisionBuilding (Variables|Components|GetCollisionBuilding) "QueryOnly"))))

(event Custom|BuildObject%20-%20Server
  (params (Target :type BP%20Collision%20Building%20Object%20Reference))
  (CallFunction|BuildObject-All Target))

(event Custom|BindonDestroyed
  (params (DestroyedActor :type Actor%20Object%20Reference))
  ;[0 0 0] Begin play
  (Utilities|IsValid (Variables|Components|GetCollisionBuilding)
    (:Is%20Valid
      (Default|ControlCollisionBuilding (Variables|Components|GetCollisionBuilding) "QueryOnly"))))

(event Custom|BuildObject%20-%20All
  (params (Target :type BP%20Collision%20Building%20Object%20Reference))
  (Variables|Engine|SetisBuildingMode false)
  (bind _output_get (Variables|Components|SetCollisionBuilding Target))
  (Utilities|IsValid _output_get
    (:Is%20Valid
      (Default|ControlCollisionBuilding _output_get "NoCollision"))
    (:Is%20Not%20Valid
      _))
  (Utilities|FlowControl|Delay 0.1)
  (CallFunction|StartWork)
  (CallFunction|RestoreMaterials)
  (Utilities|IsValid (Variables|Components|GetCollisionBuilding)
    (:Is%20Valid
      (Game|BindEventtoOnDestroyed (delegate Custom|CustomEvent)))))

(event Custom|ReplicateCanBuild%20-%20All
  (params (CanBuild :type Boolean))
  ;[0 0 0] Can Build - Event Tick
  (Variables|Engine|SetCanBuild CanBuild))

(event Custom|UpdateUpgradeInfo
  ;[0 0 0] Upgrade buildings - FUTURE UPDATE
  (bind _aswb_upgrade_building (Utilities|Casting|CastToWB_UpgradeBuilding (UserInterface|GetUserWidgetObject (Variables|Default|GetRadiusWidget))))
  (Default|UpdateCraftInfo _aswb_upgrade_building))

(event Custom|RememberMaterial%20-%20All
  (bind _returnvalue (Actor|GetComponentbyClass "/Script/Engine.ChildActorComponent"))
  ;[0 0 0] Apply materials
  (Variables|Engine|SetDefaultMeterials (Rendering|Material|GetMaterials (Variables|Default|GetStaticMesh)))
  (Utilities|IsValid _returnvalue
    (:Is%20Valid
      (bind _asbp_interact_actor (Utilities|Casting|CastToBP_InteractActor (Variables|/Script/Engine.ChildActorComponent|GetChildActor _returnvalue)))
      (Variables|Engine|SetSM_Mats (Rendering|Material|GetMaterials (Variables|/Game/ModernRPG/General/Blueprints/InteractActors/BP_InteractActor.BP_InteractActor_C|GetStaticMesh _asbp_interact_actor))))))

(event Custom|ReplicateCanBuild%20-%20Server
  ;[0 0 0] Can Build - Event Tick
  (bind _newparam (CallFunction|CheckCanBuild))
  (CallFunction|ReplicateCanBuild-All _newparam))

(event Custom|SetCurrentHealth%20-%20All
  (params (Health :type Float%20%28double-precision%29) (MaxHealth :type Float%20%28double-precision%29))
  ;[0 0 0] Event Any Damage
  (Variables|Damage|SetHealth Health)
  (Variables|Damage|SetMaxHealth MaxHealth))

(event Custom|UpdateHealth
  (params (Health :type Float%20%28double-precision%29) (DamageCauser :type Actor%20Object%20Reference))
  ;[0 0 0] Event Any Damage
  (Utilities|IsValid (Variables|Default|GetHealthWidget)
    (:Is%20Valid
      (Variables|Default|SetDamageCauser DamageCauser)
      (Rendering|SetVisibility (Variables|Default|GetHealthWidget) true false)
      (bind _aswb_health_building (Utilities|Casting|CastToWB_HealthBuilding (UserInterface|GetUserWidgetObject (Variables|Default|GetHealthWidget))))
      (bind _output_get (Variables|Damage|SetHealth Health))
      (Default|Update _aswb_health_building _output_get (.Health (Utilities|Struct|BreakS_Building (Variables|Engine|GetS_Building))))
      (if (== (Variables|Damage|GetHealth) 0.0)
        (Utilities|FlowControl|DoOnce false
          (:Completed
            (Actor|DestroyActor)))
        (else
          (Utilities|FlowControl|RetriggerableDelay 3.0)
          (Utilities|IsValid (Variables|Default|GetHealthWidget)
            (:Is%20Valid
              (Rendering|SetVisibility (Variables|Default|GetHealthWidget) false false))))))))

(event EventBeginPlay
  (bind _s_building (Variables|Engine|GetS_Building))
  (bind _health (Utilities|Struct|BreakS_Building _s_building))
  ;[0 0 0] Begin play
  (Utilities|FlowControl|Sequence
    (:then_0
      (CallFunction|RememberMaterial-All)
      (CallFunction|InitializeBuilding)
      (CallFunction|SetupWidget)
      (Utilities|Casting|CastToWB_HealthBuilding (UserInterface|GetUserWidgetObject (Variables|Default|GetHealthWidget)))
      (CallFunction|SetCurrentHealth-All _health _health))
    (:then_1
      (Variables|Engine|SetDefaultRelativeTransform (Transformation|GetRelativeTransform (Variables|Default|GetStaticMesh)))
      (Game|BindEventtoOnDestroyed (delegate Custom|BindonDestroyed))
      (Collision|SetCollisionResponsetoChannel (Variables|Default|GetStaticMesh) "ECC_GameTraceChannel7" "ECR_Overlap"))))

(event Game|Damage|EventAnyDamage
  (params (Damage :type Float%20%28single-precision%29) (DamageType :type Damage%20Type%20Object%20Reference) (InstigatedBy :type Controller%20Object%20Reference) (DamageCauser :type Actor%20Object%20Reference))
  ;[0 0 0] Event Any Damage
  (CallFunction|UpdateHealth (Math|Float|Clamp(Float) (- (Variables|Damage|GetHealth) Damage) 0.0 (Variables|Damage|GetMaxHealth)) DamageCauser))

(event EventTick
  (params (DeltaSeconds :type Float%20%28single-precision%29))
  ;[0 0 0] Can Build - Event Tick
  (if (Variables|Engine|GetisBuildingMode)
    (if (Default|CanCraft? (Actor|GetComponentbyClass (Components|GetOwner) "/Game/ModernRPG/General/Blueprints/Craft/AC_Craft.AC_Craft_C") (Utilities|Struct|BreakS_Building (Variables|Engine|GetS_Building)))
      (CallFunction|ReplicateCanBuild-Server))))

(event EventAfterInteractAction
  (params (Character :type Character%20Object%20Reference))
  ;[0 0 0] Start/Stop Item Look
  (Default|TrytoUpgrade-Server (Actor|GetComponentbyClass Character "/Game/ModernRPG/General/Blueprints/Building/AC_Building.AC_Building_C") (Variables|Engine|GetS_Building) self))

(event EventEnterRadiusI
  (params (Character :type Character%20Object%20Reference))
  ;[0 0 0] Start/Stop Item Look
  (if (not (Variables|Engine|GetisBuildingMode))
    (CallFunction|UpdateUpgradeInfo)))

(event EventStartItemLook
  (params (Character :type Character%20Object%20Reference))
  ;[0 0 0] Start/Stop Item Look
  (if (not (Variables|Engine|GetisBuildingMode))
    (CallFunction|UpdateUpgradeInfo)
    (|CallParentFunction Character)
    (else
      (|CallParentFunction Character))))

(fn ConstructionScript
  (bind _dt_building (Variables|Engine|GetDT_Building))
  (bind (_datatable _rowname) (Utilities|Struct|BreakDataTableRowHandle _dt_building))
  (Utilities|FlowControl|Sequence
    (:then_0
      (bind _returnvalue (Utilities|GetDataTableRow _datatable _rowname)
        (:then
          (Variables|Engine|SetS_Building _returnvalue))))
    (:then_1
      (Rendering|SetVisibility (Variables|Default|GetGroundChecker) (not (Variables|Settings|GetPreviewMode)) false))))

(fn OnRepCanBuild
  (CallFunction|PossibilityMaterial (Variables|Engine|GetCanBuild)))

(fn PossibilityMaterial
  (params (Possible :type Boolean))
  (bind _returnvalue (Actor|GetComponentbyClass "/Script/Engine.ChildActorComponent"))
  (bind _returnvalue_2 (select Possible "/Game/ModernRPG/Materials/Car/MI_BuildPossible.MI_BuildPossible" "/Game/ModernRPG/Materials/Car/MI_BuildImpossible.MI_BuildImpossible"))
  (bind _childactor (Variables|/Script/Engine.ChildActorComponent|GetChildActor _returnvalue))
  (for (_ _array_index) (Rendering|Material|GetMaterials (Variables|Default|GetStaticMesh))
    (Rendering|Material|SetMaterial (Variables|Default|GetStaticMesh) _array_index (select Possible "/Game/ModernRPG/Materials/Car/MI_BuildPossible.MI_BuildPossible" "/Game/ModernRPG/Materials/Car/MI_BuildImpossible.MI_BuildImpossible")))
  (Utilities|IsValid _returnvalue
    (:Is%20Valid
      (bind _asbp_interact_actor (Utilities|Casting|CastToBP_InteractActor _childactor)
        (:then
          (LocalVariables|SetFindIn _asbp_interact_actor))
        (:CastFailed
          (bind _asbp_simple_interact (Utilities|Casting|CastToBP_SimpleInteract _childactor))
          (LocalVariables|SetFindIn _asbp_simple_interact)))
      (if (Utilities|Array|IsValidIndex (Actor|GetComponentsByClass (LocalVariables|GetFindIn) "/Script/Engine.SkeletalMeshComponent"))
        (for _array_element (Actor|GetComponentsByClass (LocalVariables|GetFindIn) "/Script/Engine.SkeletalMeshComponent")
          (for (_ _array_index_2) (Rendering|Material|GetMaterials _array_element)
            (Rendering|Material|SetMaterial _array_element _array_index_2 _returnvalue_2))))
      (if (Utilities|Array|IsValidIndex (Actor|GetComponentsByClass (LocalVariables|GetFindIn) "/Script/Engine.StaticMeshComponent"))
        (for _array_element_2 (Actor|GetComponentsByClass (LocalVariables|GetFindIn) "/Script/Engine.StaticMeshComponent")
          (for (_ _array_index_3) (Rendering|Material|GetMaterials _array_element_2)
            (Rendering|Material|SetMaterial _array_element_2 _array_index_3 _returnvalue_2)))
        (return)))))

(fn FindActiveBuildings
  (params (Array :type Array%20of%20Actor%20Object%20References))
  (bind _array_element (Utilities|Array|ForEachLoopwithBreak Array :!label _label)
    (:LoopBody
      (bind _asbp_buildings_master (Utilities|Casting|CastToBP_BuildingsMaster _array_element))
      (if (Variables|BP_BuildingsMaster_C|GetisBuildingMode _asbp_buildings_master)
        (LocalVariables|SetFound true)
        (goto _label Break)))
    (:Completed
      (return (LocalVariables|GetFound)))))

(fn RestoreMaterials
  (bind _returnvalue (Actor|GetComponentbyClass "/Script/Engine.ChildActorComponent"))
  (for (_ _array_index) (Rendering|Material|GetMaterials (Variables|Default|GetStaticMesh))
    (Rendering|Material|SetMaterial (Variables|Default|GetStaticMesh) _array_index (Utilities|Array|Get(acopy) (Variables|Engine|GetDefaultMeterials) _array_index)))
  (Utilities|IsValid _returnvalue
    (:Is%20Valid
      (bind _asbp_interact_actor (Utilities|Casting|CastToBP_InteractActor (Variables|/Script/Engine.ChildActorComponent|GetChildActor _returnvalue))
        (:then
          (LocalVariables|SetFindIn _asbp_interact_actor))
        (:CastFailed
          (bind _asbp_simple_interact (Utilities|Casting|CastToBP_SimpleInteract (Variables|/Script/Engine.ChildActorComponent|GetChildActor (Actor|GetComponentbyClass "/Script/Engine.ChildActorComponent"))))
          (LocalVariables|SetFindIn _asbp_simple_interact)))
      (if (Utilities|Array|IsValidIndex (Actor|GetComponentsByClass (LocalVariables|GetFindIn) "/Script/Engine.SkeletalMeshComponent"))
        (for _array_element (Actor|GetComponentsByClass (LocalVariables|GetFindIn) "/Script/Engine.SkeletalMeshComponent")
          (for (_ _array_index_2) (Rendering|Material|GetMaterials _array_element)
            (Rendering|Material|SetMaterial _array_element _array_index_2 (Utilities|Array|Get(acopy) (Variables|Engine|GetSK_Mats) _array_index_2)))))
      (if (Utilities|Array|IsValidIndex (Actor|GetComponentsByClass (LocalVariables|GetFindIn) "/Script/Engine.StaticMeshComponent"))
        (for _array_element_2 (Actor|GetComponentsByClass (LocalVariables|GetFindIn) "/Script/Engine.StaticMeshComponent")
          (for (_ _array_index_3) (Rendering|Material|GetMaterials _array_element_2)
            (Rendering|Material|SetMaterial _array_element_2 _array_index_3 (Utilities|Array|Get(acopy) (Variables|Engine|GetSM_Mats) _array_index_3))))
        (return)))))

(fn ControlFixLocation
  (params (FixToNullCoordinates? :type Boolean))
  (if FixToNullCoordinates?
    (if (not (Variables|Engine|GetNull?))
      (Transformation|SetRelativeLocation (Variables|Default|GetStaticMesh) (Utilities|Struct|BreakS_Building (Variables|Engine|GetS_Building)) false true)
      (Variables|Engine|SetNull? true))
    (elif (Variables|Engine|GetNull?)
      (Transformation|SetRelativeLocation (Variables|Default|GetStaticMesh) (.Location (Math|Transform|BreakTransform (Variables|Engine|GetDefaultRelativeTransform))) false true)
      (Variables|Engine|SetNull? false))))

(fn InitializeBuilding
  (bind _dt_building (Variables|Engine|GetDT_Building))
  (bind (_datatable _rowname) (Utilities|Struct|BreakDataTableRowHandle _dt_building))
  (if (not (Variables|Settings|GetPre-generated?))
    (CallFunction|PossibilityMaterial (Variables|Engine|GetCanBuild))
    (Actor|Tick|SetActorTickEnabled true)
    (Variables|Engine|SetisBuildingMode true)
    (bind _returnvalue (Utilities|GetDataTableRow _datatable _rowname)
      (:then
        (bind _output_get (Variables|Engine|SetS_Building _returnvalue))
        (if (.OnlyOnTheGround (Utilities|Struct|BreakS_Building _output_get))
          (Variables|/Script/Engine.PrimitiveComponent|SetbGenerateOverlapEvents (Variables|Default|GetGroundChecker) true))))
    (else
      (CallFunction|BuildObject-All))))

(fn CheckCanBuild
  (if (Utilities|Struct|BreakS_Building (Variables|Engine|GetS_Building))
    (bind _output_get (LocalVariables|Setlocal (Collision|GetOverlappingActors (Variables|Default|GetGroundChecker) 0 :!class /Script/Engine.PrimitiveComponent)))
    (Utilities|Array|RemoveItem _output_get self)
    (if (Utilities|Array|IsValidIndex (LocalVariables|Getlocal))
      (if (Utilities|Array|IsValidIndex (Collision|GetOverlappingActors (Variables|Default|GetStaticMesh) "/Script/Engine.Pawn" :!class /Script/Engine.PrimitiveComponent)) :!label _label
        (return false)
        (else
          (bind _output_get_2 (Variables|Engine|SetOA (Collision|GetOverlappingActors (Variables|Default|GetStaticMesh) "BP_BuildingsMaster_C" :!class /Script/Engine.PrimitiveComponent) :!label _label_2))
          (if (Utilities|Array|IsValidIndex _output_get_2)
            (Utilities|Array|RemoveIndex (Variables|Engine|GetOA) (Utilities|Array|FindItem (Variables|Engine|GetOA) self))
            (if (Utilities|Array|IsValidIndex (Variables|Engine|GetOA))
              (return false)
              (else
                (return true)))
            (elif (Utilities|Array|IsValidIndex (Collision|GetOverlappingActors (Variables|Default|GetStaticMesh) "/Script/Engine.Pawn" :!class /Script/Engine.PrimitiveComponent))
              (return false)
              (else
                (return true))))))
      (else
        (bind _output_get_3 (LocalVariables|SetCB (Collision|GetOverlappingActors (Variables|Default|GetStaticMesh) "/Game/ModernRPG/General/Blueprints/Building/Components/BP_CollisionBuilding.BP_CollisionBuilding_C" :!class /Script/Engine.PrimitiveComponent)))
        (if (Utilities|Array|IsValidIndex _output_get_3)
          (bind _array_element (Utilities|Array|ForEachLoopwithBreak (LocalVariables|GetCB) :!label _label_3)
            (:LoopBody
              (bind _asbp_collision_building (Utilities|Casting|CastToBP_CollisionBuilding _array_element))
              (if (Utilities|Array|ContainsItem (Variables|/Game/ModernRPG/General/Blueprints/Building/Components/BP_CollisionBuilding.BP_CollisionBuilding_C|GetPermittedBuildings _asbp_collision_building) (.BuildingType (Utilities|Struct|BreakS_Building (Variables|Engine|GetS_Building))))
                (Utilities|FlowControl|Sequence
                  (:then_0
                    (goto _label_3 Break))
                  (:then_1
                    (LocalVariables|SetFound true)))))
            (:Completed
              (if (LocalVariables|GetFound)
                (goto _label_2)
                (else
                  (return false)))))
          (else
            (return false)))))
    (else
      (goto _label))))

(fn SettoNullCoordinatesPreview
  (params (NewRelativeRotation :type Rotator))
  (Transformation|SetRelativeLocation (Variables|Default|GetStaticMesh) (Utilities|Struct|BreakS_Building (Variables|Engine|GetS_Building)) false true)
  (Transformation|SetActorRotation NewRelativeRotation)
  (for (_ _array_index) (Rendering|Material|GetMaterials (Variables|Default|GetStaticMesh))
    (Rendering|Material|SetMaterial (Variables|Default|GetStaticMesh) _array_index "/Game/ModernRPG/Materials/Car/MI_Preview.MI_Preview"))
  (return))

(fn StartWork
  (for _array_element (Actor|GetComponentsByClass "/Script/Engine.ChildActorComponent")
    (bind _asbp_collision_building (Utilities|Casting|CastToBP_CollisionBuilding (Variables|/Script/Engine.ChildActorComponent|GetChildActor _array_element)))
    (Default|ControlCollisionBuilding _asbp_collision_building "QueryOnly")
    (Rendering|SetActorHiddenInGame _asbp_collision_building false))
  (Actor|Tick|SetActorTickEnabled false)
  (Collision|SetCollisionEnabled (Variables|Default|GetStaticMesh) "QueryAndPhysics")
  (CallFunction|ControlCollision "QueryAndPhysics")
  (Collision|SetCollisionResponsetoAllChannels (Variables|Default|GetStaticMesh) "ECR_Block")
  (Collision|SetCollisionResponsetoChannel (Variables|Default|GetStaticMesh) "ECC_GameTraceChannel7" "ECR_Overlap")
  (Collision|SetCollisionResponsetoChannel (Variables|Default|GetStaticMesh) "ECC_WorldDynamic" "ECR_Overlap")
  (Collision|SetCollisionResponsetoChannel (Variables|Default|GetStaticMesh) "ECC_GameTraceChannel18" "ECR_Ignore")
  (Collision|SetCollisionEnabled (Variables|Default|GetGroundChecker) "NoCollision")
  (if (Utilities|Struct|BreakS_Building (Variables|Engine|GetS_Building))
    (Collision|SetCollisionResponsetoChannel (Variables|Default|GetInteractArea) "ECC_GameTraceChannel5" "ECR_Block")
    (else
      (Collision|SetCollisionResponsetoChannel (Variables|Default|GetStaticMesh) "ECC_GameTraceChannel5" "ECR_Ignore")))
  (CallFunction|Start))