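; BP_SoundTraps is a hanging noise trap that plays a sound and reports an AI noise event when a player-controlled pawn overlaps its box, then pauses briefly before it can retrigger.
; Interacting cuts it down, disabling the trigger, breaking the physics constraint, detaching the cable and nudging the mesh with a random impulse.
; The cut mesh ignores pawns and plays a quieter hit sound once on impact.
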(event OnComponentBeginOverlap(Box)
  (params (OverlappedComponent :type Primitive%20Component%20Object%20Reference) (OtherActor :type Actor%20Object%20Reference) (OtherComp :type Primitive%20Component%20Object%20Reference) (OtherBodyIndex :type Integer) (bFromSweep :type Boolean) (SweepResult :type Hit%20Result%20Structure%20%28by%20ref%29))
  (bind _returnvalue (Transformation|GetActorLocation))
  ;[1 1 1] On Overlapped
  (bind _aspawn (Utilities|Casting|CastToPawn OtherActor))
  (if (not (Variables|Default|GetbCut))
    (if (Pawn|IsPlayerControlled _aspawn)
      (if (not (Variables|Default|GetOverlapDelay))
        (Variables|Default|SetOverlapDelay true)
        (Audio|PlaySoundatLocation (Variables|Settings|GetOverlapSound) _returnvalue "0, 0, 0" 1.0 1.0 0.0 0 0 0 0)
        (Class|AISenseHearing|ReportNoiseEvent _returnvalue 1.0 _aspawn (Variables|Settings|GetNoiseRange) "Noise")
        (Utilities|FlowControl|Delay 5.0)
        (Variables|Default|SetOverlapDelay false)))))

(event OnComponentHit(PhysicsMesh)
  (params (HitComponent :type Primitive%20Component%20Object%20Reference) (OtherActor :type Actor%20Object%20Reference) (OtherComp :type Primitive%20Component%20Object%20Reference) (NormalImpulse :type Vector :default "0, 0, 0") (Hit :type Hit%20Result%20Structure%20%28by%20ref%29))
  ;[1 1 1] Hit the ground
  (if (Variables|Default|GetbCut)
    (Utilities|FlowControl|DoOnce false
      (:Completed
        (Audio|PlaySoundatLocation (Variables|Settings|GetHitSound) (Transformation|GetActorLocation) "0, 0, 0" 0.2 1.0 0.0 0 0 0 0)))))

(event Custom|Cut
  (bind _returnvalue (Math|Random|RandomUnitVector))
  (bind _returnvalue_2 (* _returnvalue 1e+01))
  (bind (_x _y) (Math|Vector|BreakVector _returnvalue_2))
  ;[1 1 1] Cut the rope
  (Variables|Default|SetBusy true)
  (Variables|Default|SetbCut true)
  (Physics|AddImpulse (Variables|Default|GetPhysicsMesh) (Math|Vector|MakeVector _x _y -1.0) "None" true)
  (Class|PhysicsConstraintComponent|BreakConstraint (Variables|Default|GetPhysicsConstraint))
  (Class|CableComponent|SetAttachEndto (Variables|Default|GetCable) 0 "None" "None")
  (Collision|SetCollisionResponsetoChannel (Variables|Default|GetPhysicsMesh) "ECC_Pawn" "ECR_Ignore"))

(event EventInteract
  (params (Character :type Character%20Object%20Reference))
  ;[1 1 1] Cut on interact
  (CallFunction|Cut))

(fn ConstructionScript
  (Components|StaticMesh|SetStaticMesh (Variables|Default|GetPhysicsMesh) (Variables|Settings|GetMesh)))